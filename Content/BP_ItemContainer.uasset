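; Interactable item container that the player opens to take items into their inventory.
; Interact opens it and pushes an input context on the interactor's ContextComponent, with the container as input receiver.
; While receiving input, the Interact tag advances the widget selection and the Jump tag moves the selected slot into player 0's InventoryComponent.
; Take-all, close and context removal logic exists but is unconnected, so nothing here closes the container.
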(event EventBeginPlay)

(event Collision|EventActorBeginOverlap
  (params (OtherActor :type Actor%20Object%20Reference)))

(event EventTick
  (params (DeltaSeconds :type Float%20%28single-precision%29)))

(event EventHandleInput
  (params (Tag :type Gameplay%20Tag%20Structure) (Value :type Input%20Action%20Value%20Structure%20%28by%20ref%29) (TriggerEvent :type ETriggerEvent%20Enum :default "None"))
  (|SwitchGameplayTag Tag
    (:Action.Interact
      (Class|ContainerWidgetBase|MoveSelection (Variables|Default|GetNewVar) 1))
    (:Action.Jump
      (Class|ItemContainer|TakeSlot (Class|ContainerWidgetBase|GetSelectedSlotIndex (Class|ItemContainer|GetActiveWidget)) (Actor|GetComponentbyClass (Game|Player|GetPlayerPawn 0) "/Script/InventorySystem.InventoryComponent")))))

(event EventInteract
  (params (Interactor :type Actor%20Object%20Reference))
  (bind _returnvalue (Actor|GetComponentbyClass Interactor "/Script/ContextFramework.ContextComponent"))
  (Class|ItemContainer|Open)
  (Utilities|IsValid _returnvalue
    (:Is%20Valid
      (if true
        (bind _returnvalue_2 (Class|ContextComponent|AddContext _returnvalue (Utilities|Struct|MakeActiveContext "(Guid=00000000000000000000000000000000)" "/Game/DA_ChallengeDa.DA_ChallengeDa" "(EnterMontage=None,ExitMontage=None,SnapTarget=None,LookTarget=None)" 0 0 self)))))))

(fn ConstructionScript)

(fn GetInteractionDisplayName
  (return "Interact"))