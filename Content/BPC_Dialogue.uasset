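; BPC_Dialogue shows dialogue lines on screen through a WBP_DialogueTest widget.
; When a line starts, it removes any existing widget, then creates a new one for player 0 with the speaker name, line text and a reference to itself.
; The widget is stored and added to the viewport, then removed when the dialogue ends.
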(event EventBeginPlay)

(event EventTick
  (params (DeltaSeconds :type Float%20%28single-precision%29)))

(event EventOnLineStarted
  (params (Line :type Dialogue%20Line%20Structure%20%28by%20ref%29))
  (bind (_speakername _linetext) (Utilities|Struct|BreakDialogueLine Line))
  (bind _newvar (Variables|Default|GetNewVar)
    (:then
      (Widget|RemovefromParent _newvar))
    (:else
      _))
  (bind _returnvalue (UserInterface|CreateWidget "/Game/WBP_DialogueTest.WBP_DialogueTest_C" (Game|GetPlayerController 0) self _speakername _linetext))
  (bind _output_get (Variables|Default|SetNewVar _returnvalue))
  (UserInterface|Viewport|AddtoViewport _returnvalue 0))

(event EventOnDialogueEnded
  (Widget|RemovefromParent (Variables|Default|GetNewVar)))