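; Gameplay ability that attacks with the shooter character's current weapon until input is released.
; It commits, calls the weapon's attack, then re-commits on each Weapon.Fire event.
; Shots play a montage rate-scaled to attack rate, with damage awaiting Event.Weapon.Attack, or deal damage directly without one.
; Damage is a GE_DealDamages spec with a set-by-caller magnitude from an avatar attribute, passed to the weapon's PerformAttack.
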(event Custom|Attack
  ;[0.15 0.15 0.15 0.5] Attack Launch
  (if (not (Variables|Default|GetListeningForAttack_0))
    (Variables|Default|SetListeningForAttack_0 true)
    (Ability|Tasks|WaitGameplayEvent "(TagName=\"Event.Weapon.Attack\")" 0
      (:EventReceived
        (CallFunction|DealDamages)))))

(event Custom|DealDamages
  (bind _result (Math|Float|NegateFloat (.ReturnValue (Ability|Attribute|GetFloatAttribute (Ability|GetAvatarActorfromActorInfo) "(AttributeName=\"Damage\",Attribute=/Script/Millionnaires.BaseAttributeSet:Damage,AttributeOwner=\"/Script/CoreUObject.Class'/Script/Millionnaires.BaseAttributeSet'\")")))
    (:%20%20
      (bind _returnvalue (Ability|GameplayEffect|AssignTagSetbyCallerMagnitude (Ability|MakeOutgoingGameplayEffectSpec "/Game/02_Blueprints/GameplayAbilitySystem/Effects/GE_DealDamages.GE_DealDamages_C") "(TagName=\"Damage.Calculation\")" _result))
      (Class|WeaponBase|PerformAttack (Variables|Default|GetUsedWeapon) _returnvalue))))

(event Custom|AttackTrigger
  (bind _usedweapon (Variables|Default|GetUsedWeapon))
  (bind _weapondata (Variables|/Script/Millionnaires.WeaponBase|GetWeaponData _usedweapon))
  (bind _attackmontage (Variables|/Script/Millionnaires.WeaponData|GetAttackMontage _weapondata))
  ;[0.15 0.15 0.15 0.5] Start Attack
  (if (not (Variables|Default|GetListeningForAttack))
    (Variables|Default|SetListeningForAttack true)
    (Class|WeaponBase|CallAttack (Variables|Default|GetUsedWeapon))
    (Ability|Tasks|WaitGameplayEvent "(TagName=\"Weapon.Fire\")" 0
      (:then
        (Utilities|IsValid _attackmontage :!label _label
          (:Is%20Valid
            (|PlayMontageandWaitProxy "None" _attackmontage (* (Variables|/Script/Millionnaires.WeaponData|GetAttackRate _weapondata) (Animation|GetPlayLength _attackmontage)) "None" false 1.0 0.0 false
              (:then
                (CallFunction|ATTACK))))
          (:Is%20Not%20Valid
            (CallFunction|DealDamages))))
      (:EventReceived
        (bind _returnvalue (Ability|CommitAbility))
        (if _returnvalue
          (goto _label))))))

(event Ability|EventActivateAbility
  (bind _returnvalue (Ability|CommitAbility))
  (if _returnvalue
    (bind _asbp_shooter_character (Utilities|Casting|CastToBP_ShooterCharacter (Ability|GetAvatarActorfromActorInfo)))
    (bind _currentweapon (Variables|/Game/Variant_Shooter/Blueprints/BP_ShooterCharacter.BP_ShooterCharacter_C|GetCurrentWeapon _asbp_shooter_character)
      (:then
        (bind _output_get (Variables|Default|SetUsedWeapon _currentweapon))
        (bind _returnvalue_2 (Class|WeaponBase|CanAttack _output_get))
        (if _returnvalue_2
          (Ability|Tasks|WaitInputRelease false
            (:then
              (CallFunction|AttackTrigger))
            (:OnRelease
              (Class|WeaponBase|StopAttacking (Variables|Default|GetUsedWeapon))
              (Ability|EndAbility)))
          (else
            (Ability|EndAbility))))
      (:else))
    (else
      (Ability|EndAbility))))

(event Ability|EventOnEndAbility
  (params (bWasCancelled :type Boolean)))