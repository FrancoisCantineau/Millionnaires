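; Gameplay Ability that reloads an AI character's equipped weapon instantly on activation, with no montage or delay.
; It applies GE_WeaponReload to the weapon actor found through the avatar's WeaponsManagerComponent, passing a fixed SetByCaller reload amount.
; It then removes the non-replicated loose State.Ammo.Empty tag from the avatar and ends.
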(event Ability|EventActivateAbility
  (bind _returnvalue (Ability|GameplayEffect|AssignTagSetbyCallerMagnitude (Ability|MakeOutgoingGameplayEffectSpec "/Game/02_Blueprints/GameplayAbilitySystem/Effects/GE_WeaponReload.GE_WeaponReload_C") "(TagName=\"Data.Weapon.ReloadValue\")" 1e+01))
  (GameplayEffects|ApplyGameplayEffectSpecToTarget _returnvalue (Ability|TargetData|AbilityTargetDatafromActor (Variables|/Script/Millionnaires.WeaponsManagerComponent|GetEquippedWeapon (Actor|GetComponentbyClass (Ability|GetAvatarActorfromActorInfo) "/Script/Millionnaires.WeaponsManagerComponent"))))
  (Ability|GameplayEffect|RemoveLooseGameplayTags (Ability|GetAvatarActorfromActorInfo) (GameplayTags|MakeGameplayTagContainerfromTag "(TagName=\"State.Ammo.Empty\")"))
  (Ability|EndAbility))

(event Ability|EventOnEndAbility
  (params (bWasCancelled :type Boolean)))