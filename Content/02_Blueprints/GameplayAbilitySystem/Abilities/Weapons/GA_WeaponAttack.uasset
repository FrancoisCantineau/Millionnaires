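; Gameplay ability that fires the avatar's equipped weapon, looping at an attribute-driven rate for full-auto weapons until input release.
; Each shot passes an attribute check, calls the weapon's attack, then applies a cost effect to the weapon's own ASC on the Weapon.Fire event.
; Damage follows montage gameplay events, or is immediate without a montage, passing a SetByCaller spec scaled by event magnitude to the weapon.
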(event Custom|Attack
  ;[0.15 0.15 0.15 0.5] Attack Launch
  (Ability|Tasks|WaitGameplayEvent "(TagName=\"Event.Weapon.Attack\")" 0 true
    (:then
      (Ability|Tasks|WaitGameplayEvent "(TagName=\"Event.HitScan.Start\")" 0 true
        (:then
          (Ability|Tasks|WaitGameplayEvent "(TagName=\"Event.HitScan.End\")" 0 true
            (:EventReceived
              (Class|WeaponBase|InterruptAttack (Variables|Default|GetUsedWeapon)))))
        (:EventReceived
          (Development|PrintString "IOGSEOI")
          (CallFunction|DealDamages))))
    (:EventReceived
      (CallFunction|DealDamages))))

(event Custom|DealDamages
  (bind _usedweapon (Variables|Default|GetUsedWeapon))
  (bind _returnvalue (Ability|Attribute|GetFloatAttribute _usedweapon "(AttributeName=\"WeaponDamage\",Attribute=/Script/Millionnaires.WeaponAttributeSet:WeaponDamage,AttributeOwner=\"/Script/CoreUObject.Class'/Script/Millionnaires.WeaponAttributeSet'\")"))
  (bind _result (Math|Float|NegateFloat (* (Variables|Default|GetEvent%20Magnitude) _returnvalue))
    (:%20%20
      (Development|PrintString (Utilities|String|ToString(Float) _returnvalue))
      (bind _returnvalue_2 (Ability|GameplayEffect|AssignTagSetbyCallerMagnitude (Ability|MakeOutgoingGameplayEffectSpec "/Game/02_Blueprints/GameplayAbilitySystem/Effects/GE_DealDamages.GE_DealDamages_C") "(TagName=\"Damage.Calculation\")" _result))
      (Class|WeaponBase|PerformAttack (Variables|Default|GetUsedWeapon) _returnvalue_2))))

(event Custom|AttackTrigger
  (bind _usedweapon (Variables|Default|GetUsedWeapon))
  (bind _usedweapon_2 (Variables|Default|GetUsedWeapon))
  (bind _returnvalue (Ability|Attribute|GetFloatAttribute _usedweapon_2 "(AttributeName=\"AttackRate\",Attribute=/Script/Millionnaires.WeaponAttributeSet:AttackRate,AttributeOwner=\"/Script/CoreUObject.Class'/Script/Millionnaires.WeaponAttributeSet'\")"))
  (bind _weapondata (Variables|/Script/Millionnaires.WeaponBase|GetWeaponData _usedweapon))
  (bind _attackmontage (Variables|/Script/Millionnaires.WeaponData|GetAttackMontage _weapondata))
  (bind _returnvalue_2 (Animation|GetPlayLength _attackmontage))
  (bind _returnvalue_3 (* _returnvalue _returnvalue_2))
  ;[0.15 0.15 0.15 0.5] Start Attack
  (if (> (.ReturnValue (Ability|Attribute|GetFloatAttribute (Variables|Default|GetUsedWeapon) "(AttributeName=\"AmmoInMag\",Attribute=/Script/Millionnaires.WeaponAttributeSet:AmmoInMag,AttributeOwner=\"/Script/CoreUObject.Class'/Script/Millionnaires.WeaponAttributeSet'\")")) 0.0)
    (bind _payload (Ability|Tasks|WaitGameplayEvent "(TagName=\"Weapon.Fire\")" 0 true)
      (:then
        (Class|WeaponBase|CallAttack (Variables|Default|GetUsedWeapon)))
      (:EventReceived
        (Variables|Default|SetEvent%20Magnitude (Utilities|Struct|BreakGameplayEventData _payload))
        (GameplayEffects|ApplyGameplayEffectToSelf :self (Variables|/Script/Millionnaires.WeaponBase|GetAbilitySystemComponent (Variables|Default|GetUsedWeapon)) :GameplayEffectClass "/Game/02_Blueprints/GameplayAbilitySystem/Effects/GE_WeaponAttackCost.GE_WeaponAttackCost_C")
        (Utilities|IsValid _attackmontage
          (:Is%20Valid
            (Development|PrintString (Utilities|String|ToString(Float) _returnvalue_3))
            (|PlayMontageandWaitProxy "None" _attackmontage _returnvalue_3 "None" false 1.0 0.0 false
              (:then
                (CallFunction|ATTACK))))
          (:Is%20Not%20Valid
            (CallFunction|DealDamages)))))
    (else
      (Audio|PlaySound2D "/Engine/VREditor/Sounds/UI/Flashlight_Switch.Flashlight_Switch" 1.0 1.0 0.0 0 0))))

(event Custom|FireLoop
  (CallFunction|AttackTrigger)
  (Ability|Tasks|WaitDelay (/ 1 (.ReturnValue (Ability|Attribute|GetFloatAttribute (Variables|Default|GetUsedWeapon) "(AttributeName=\"AttackRate\",Attribute=/Script/Millionnaires.WeaponAttributeSet:AttackRate,AttributeOwner=\"/Script/CoreUObject.Class'/Script/Millionnaires.WeaponAttributeSet'\")")))
    (:OnFinish
      (CallFunction|FireLoop))))

(event Ability|EventActivateAbility
  (bind _returnvalue (Ability|GetAvatarActorfromActorInfo))
  (bind _returnvalue_2 (Actor|GetComponentbyClass _returnvalue "/Script/Millionnaires.WeaponsManagerComponent"))
  (bind _equippedweapon (Variables|/Script/Millionnaires.WeaponsManagerComponent|GetEquippedWeapon _returnvalue_2))
  (Variables|Default|SetShotshots 0)
  (Utilities|IsValid _equippedweapon
    (:Is%20Valid
      (Variables|Default|SetUsedWeapon _equippedweapon)
      (bind _usedweapon (Variables|Default|GetUsedWeapon)
        (:then
          (bind _returnvalue_3 (Class|WeaponBase|CanAttack _usedweapon))
          (if _returnvalue_3
            (Ability|Tasks|WaitInputRelease false
              (:then
                (if (Variables|/Script/Millionnaires.WeaponData|GetbFullAuto (Variables|/Script/Millionnaires.WeaponBase|GetWeaponData (Variables|Default|GetUsedWeapon)))
                  (CallFunction|FireLoop)
                  (else
                    (CallFunction|AttackTrigger))))
              (:OnRelease
                (Class|WeaponBase|StopAttacking (Variables|Default|GetUsedWeapon))
                (Ability|EndAbility)))
            (else
              (Ability|EndAbility))))
        (:else
          (Ability|EndAbility))))))