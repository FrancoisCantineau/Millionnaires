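; Gameplay ability for AI weapon attacks, firing the avatar's equipped weapon once or in a repeating full-auto loop.
; AttackTrigger checks a weapon attribute, tagging the avatar ammo-empty on failure, otherwise calls the weapon's attack and awaits a fire event to apply cost and play the montage.
; Gameplay events then drive hit-scan interruption and ability end.
; DealDamages is an empty stub, with its SetByCaller damage logic left disconnected.
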(event Custom|Attack
  ;[0.15 0.15 0.15 0.5] Attack Launch
  (Ability|Tasks|WaitGameplayEvent "(TagName=\"Event.Weapon.Attack.Start\")" 0 true
    (:then
      (Ability|Tasks|WaitGameplayEvent "(TagName=\"Event.HitScan.Start\")" 0 true
        (:then
          (Ability|Tasks|WaitGameplayEvent "(TagName=\"Event.HitScan.End\")" 0 true
            (:then
              (Ability|Tasks|WaitGameplayEvent "(TagName=\"Event.Weapon.Attack.End\")" 0 true
                (:EventReceived
                  (Variables|Default|SetAttackOngoing false)
                  (CallFunction|EndAttack))))
            (:EventReceived
              (Class|WeaponBase|InterruptAttack (Variables|Default|GetUsedWeapon)))))
        (:EventReceived
          (CallFunction|DealDamages))))
    (:EventReceived
      (CallFunction|DealDamages))))

(event Custom|DealDamages)

(event Custom|AttackTrigger
  (bind _usedweapon (Variables|Default|GetUsedWeapon))
  (bind _weapondata (Variables|/Script/Millionnaires.WeaponBase|GetWeaponData _usedweapon))
  (bind _attackmontage (Variables|/Script/Millionnaires.WeaponData|GetAttackMontage _weapondata))
  ;[0.15 0.15 0.15 0.5] Start Attack
  (if (> (.ReturnValue (Ability|Attribute|GetFloatAttribute (Variables|Default|GetUsedWeapon) "(AttributeName=\"AmmoInMag\",Attribute=/Script/Millionnaires.WeaponAttributeSet:AmmoInMag,AttributeOwner=\"/Script/CoreUObject.Class'/Script/Millionnaires.WeaponAttributeSet'\")")) 0.0)
    (Variables|Default|SetAttackOngoing true)
    (bind _payload (Ability|Tasks|WaitGameplayEvent "(TagName=\"Weapon.Fire\")" 0 true)
      (:then
        (Class|WeaponBase|CallAttack (Variables|Default|GetUsedWeapon)))
      (:EventReceived
        (Variables|Default|SetEvent%20Magnitude (Utilities|Struct|BreakGameplayEventData _payload))
        (GameplayEffects|ApplyGameplayEffectToSelf :self (Variables|/Script/Millionnaires.WeaponBase|GetAbilitySystemComponent (Variables|Default|GetUsedWeapon)) :GameplayEffectClass "/Game/02_Blueprints/GameplayAbilitySystem/Effects/GE_WeaponAttackCost.GE_WeaponAttackCost_C")
        (Utilities|IsValid _attackmontage
          (:Is%20Valid
            (|PlayMontageandWaitProxy "None" _attackmontage (* (.ReturnValue (Ability|Attribute|GetFloatAttribute (Variables|Default|GetUsedWeapon) "(AttributeName=\"AttackRate\",Attribute=/Script/Millionnaires.WeaponAttributeSet:AttackRate,AttributeOwner=\"/Script/CoreUObject.Class'/Script/Millionnaires.WeaponAttributeSet'\")")) (Animation|GetPlayLength _attackmontage)) "None" false 1.0 0.0 false
              (:then
                (CallFunction|ATTACK))))
          (:Is%20Not%20Valid
            (CallFunction|DealDamages)))))
    (else
      (Audio|PlaySound2D "/Engine/VREditor/Sounds/UI/Flashlight_Switch.Flashlight_Switch" 1.0 1.0 0.0 0 0)
      (Ability|GameplayEffect|AddLooseGameplayTags (Ability|GetAvatarActorfromActorInfo) (GameplayTags|MakeGameplayTagContainerfromTag "(TagName=\"State.Ammo.Empty\")")))))

(event Custom|EndAttack
  (Ability|EndAbility))

(event Custom|FireLoop
  (CallFunction|AttackTrigger)
  (Ability|Tasks|WaitDelay (/ 1 (.ReturnValue (Ability|Attribute|GetFloatAttribute (Variables|Default|GetUsedWeapon) "(AttributeName=\"AttackRate\",Attribute=/Script/Millionnaires.WeaponAttributeSet:AttackRate,AttributeOwner=\"/Script/CoreUObject.Class'/Script/Millionnaires.WeaponAttributeSet'\")")))
    (:OnFinish
      (if (not (Variables|Default|GetInputReleased))
        (CallFunction|FireLoop)))))

(event Ability|EventActivateAbility
  (bind _returnvalue (Ability|GetAvatarActorfromActorInfo))
  (bind _returnvalue_2 (Actor|GetComponentbyClass _returnvalue "/Script/Millionnaires.WeaponsManagerComponent"))
  (bind _equippedweapon (Variables|/Script/Millionnaires.WeaponsManagerComponent|GetEquippedWeapon _returnvalue_2))
  (Ability|CommitAbility)
  (Variables|Default|SetAttackOngoing false)
  (Variables|Default|SetShotshots 0)
  (Utilities|IsValid _equippedweapon
    (:Is%20Valid
      (Variables|Default|SetUsedWeapon _equippedweapon)
      (Variables|Default|GetUsedWeapon
        (:then
          (if true
            (if (Variables|/Script/Millionnaires.WeaponData|GetbFullAuto (Variables|/Script/Millionnaires.WeaponBase|GetWeaponData (Variables|Default|GetUsedWeapon)))
              (CallFunction|FireLoop)
              (else
                (CallFunction|AttackTrigger)))
            (else
              (Ability|EndAbility))))
        (:else
          (Ability|EndAbility))))))