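; Gameplay ability for AI weapon attacks, using the avatar's equipped weapon from its WeaponsManagerComponent.
; After commit and CanAttack checks, it applies the attack cost, calls the weapon's attack and listens for Weapon.Fire events.
; It plays the attack montage at a rate scaled by a weapon attribute, or deals damage directly without one.
; Damage is a SetByCaller GE_DealDamages spec passed to the weapon's PerformAttack.
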(event Custom|Attack
  ;[0.15 0.15 0.15 0.5] Attack Launch
  (if (not (Variables|Default|GetListeningForAttack_0))
    (Variables|Default|SetListeningForAttack_0 true)
    (Ability|Tasks|WaitGameplayEvent "(TagName=\"Event.Weapon.Attack\")" 0
      (:then
        (Class|WeaponBase|StopAttacking (Variables|Default|GetUsedWeapon))
        (Ability|EndAbility))
      (:EventReceived
        (CallFunction|DealDamages)))))

(event Custom|DealDamages
  (bind _result (Math|Float|NegateFloat (.ReturnValue (Ability|Attribute|GetFloatAttribute (Variables|Default|GetUsedWeapon) "(AttributeName=\"WeaponDamage\",Attribute=/Script/Millionnaires.WeaponAttributeSet:WeaponDamage,AttributeOwner=\"/Script/CoreUObject.Class'/Script/Millionnaires.WeaponAttributeSet'\")")))
    (:%20%20
      (bind _returnvalue (Ability|GameplayEffect|AssignTagSetbyCallerMagnitude (Ability|MakeOutgoingGameplayEffectSpec "/Game/02_Blueprints/GameplayAbilitySystem/Effects/GE_DealDamages.GE_DealDamages_C") "(TagName=\"Damage.Calculation\")" _result))
      (Class|WeaponBase|PerformAttack (Variables|Default|GetUsedWeapon) _returnvalue))))

(event Custom|AttackTrigger
  (bind _usedweapon (Variables|Default|GetUsedWeapon))
  (bind _weapondata (Variables|/Script/Millionnaires.WeaponBase|GetWeaponData _usedweapon))
  (bind _attackmontage (Variables|/Script/Millionnaires.WeaponData|GetAttackMontage _weapondata))
  ;[0.15 0.15 0.15 0.5] Start Attack
  (GameplayEffects|ApplyGameplayEffectToSelf :self (Variables|/Script/Millionnaires.WeaponBase|GetAbilitySystemComponent (Variables|Default|GetUsedWeapon)) :GameplayEffectClass "/Game/02_Blueprints/GameplayAbilitySystem/Effects/GE_WeaponAttackCost.GE_WeaponAttackCost_C")
  (Class|WeaponBase|CallAttack (Variables|Default|GetUsedWeapon))
  (Ability|Tasks|WaitGameplayEvent "(TagName=\"Weapon.Fire\")" 0
    (:then
      (Utilities|IsValid _attackmontage :!label _label
        (:Is%20Valid
          (|PlayMontageandWaitProxy "None" _attackmontage (* (/ 1 (.ReturnValue (Ability|Attribute|GetFloatAttribute (Variables|Default|GetUsedWeapon) "(AttributeName=\"AttackRate\",Attribute=/Script/Millionnaires.WeaponAttributeSet:AttackRate,AttributeOwner=\"/Script/CoreUObject.Class'/Script/Millionnaires.WeaponAttributeSet'\")"))) (Animation|GetPlayLength _attackmontage)) "None" false 1.0 0.0 false
            (:OnCompleted
              (Ability|EndAbility))))
        (:Is%20Not%20Valid
          (CallFunction|DealDamages))))
    (:EventReceived
      (GameplayEffects|ApplyGameplayEffectToSelf :self (Variables|/Script/Millionnaires.WeaponBase|GetAbilitySystemComponent (Variables|Default|GetUsedWeapon)) :GameplayEffectClass "/Game/02_Blueprints/GameplayAbilitySystem/Effects/GE_WeaponAttackCost.GE_WeaponAttackCost_C")
      (if true
        (goto _label)))))

(event Ability|EventActivateAbility
  (bind _returnvalue (Ability|GetAvatarActorfromActorInfo))
  (bind _returnvalue_2 (Actor|GetComponentbyClass _returnvalue "/Script/Millionnaires.WeaponsManagerComponent"))
  (bind _equippedweapon (Variables|/Script/Millionnaires.WeaponsManagerComponent|GetEquippedWeapon _returnvalue_2))
  (bind _returnvalue_3 (Ability|CommitAbility))
  (if _returnvalue_3
    (Utilities|IsValid _equippedweapon
      (:Is%20Valid
        (Variables|Default|SetUsedWeapon _equippedweapon)
        (bind _usedweapon (Variables|Default|GetUsedWeapon)
          (:then
            (bind _returnvalue_4 (Class|WeaponBase|CanAttack _usedweapon))
            (if _returnvalue_4
              (CallFunction|AttackTrigger)
              (else
                (Ability|EndAbility))))
          (:else
            (Ability|EndAbility)))))
    (else
      (Ability|EndAbility))))