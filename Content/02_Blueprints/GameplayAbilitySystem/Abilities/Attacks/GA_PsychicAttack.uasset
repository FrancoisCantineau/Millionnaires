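; GA_PsychicAttack is an AI gameplay ability that inflicts a psychosis state on the AI controller's global target.
; Activation applies a using-ability effect to the owner, commits, waits a frame, then applies GE_PsychoseState to the target if it has an ability system component.
; An out-of-range gameplay event removes the target's effect and ends the ability.
; Ending the ability removes the owner's effect.
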(event Ability|EventActivateAbility
  (bind _returnvalue (Ability|ApplyGameplayEffectToOwner "/Game/02_Blueprints/GameplayAbilitySystem/Effects/GE_UsingAbility.GE_UsingAbility_C"))
  (Variables|Default|SetNewVar _returnvalue)
  (Ability|CommitAbility)
  (Utilities|FlowControl|DelayUntilNextFrame)
  (bind _targetactor (Class|BPICombatInterface|GetGlobalTarget(Message) (AI|GetAIController (Ability|GetAvatarActorfromActorInfo))))
  (Utilities|IsValid (Ability|GetAbilitySystemComponent _targetactor)
    (:Is%20Valid
      (bind _returnvalue_2 (GameplayEffects|ApplyGameplayEffectToTarget :self (Ability|GetAbilitySystemComponent (Ability|GetAvatarActorfromActorInfo)) :GameplayEffectClass "/Game/02_Blueprints/GameplayAbilitySystem/Effects/GE_PsychoseState.GE_PsychoseState_C" :Target (Ability|GetAbilitySystemComponent _targetactor)))
      (Ability|Tasks|WaitGameplayEvent "(TagName=\"Event.Ability.OutOfRange\")" 0 true false
        (:EventReceived
          (GameplayEffects|RemoveActiveGameplayEffect (Ability|GetAbilitySystemComponent _targetactor) _returnvalue_2 -1)
          (Ability|EndAbility))))))

(event Ability|EventOnEndAbility
  (params (bWasCancelled :type Boolean))
  (bind _returnvalue (Ability|GetAvatarActorfromActorInfo))
  (bind _returnvalue_2 (Ability|GetAbilitySystemComponent _returnvalue))
  (Utilities|IsValid _returnvalue_2
    (:Is%20Valid
      (GameplayEffects|RemoveActiveGameplayEffect _returnvalue_2 (Variables|Default|GetNewVar) -1))))

(event Ability|EventActivateAbilityFromEvent
  (params (EventData :type Gameplay%20Event%20Data%20Structure%20%28by%20ref%29)))