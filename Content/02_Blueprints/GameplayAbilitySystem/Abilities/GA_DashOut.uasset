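; GA_DashOut is a Gameplay Ability that dashes an AI-controlled avatar toward a target point supplied by its AI controller.
; Standard activation commits the ability, applies GE_UsingAbility and caches the point; event activation skips straight to the dash.
; A brief constant root-motion force uses clamped distance as strength and keeps its velocity on finish, with a debug print of that value.
; The ability ends when the force finishes, removing the effect.
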(event Ability|EventActivateAbility
  (bind _returnvalue (Ability|GetAvatarActorfromActorInfo))
  (bind _returnvalue_2 (Transformation|GetActorLocation _returnvalue))
  (bind _returnvalue_3 (Ability|CommitAbility))
  (if _returnvalue_3
    (bind _returnvalue_4 (Ability|ApplyGameplayEffectToOwner "/Game/02_Blueprints/GameplayAbilitySystem/Effects/GE_UsingAbility.GE_UsingAbility_C"))
    (Variables|Default|SetNewVar _returnvalue_4)
    (bind _targetpoint (Class|BPICombatInterface|GetTargetPoint(Message) (AI|GetAIController (Ability|GetAvatarActorfromActorInfo))))
    (Development|PrintString (Utilities|String|ToString(Float) (Math|Float|Clamp(Float) (Math|Vector|Distance(Vector) _returnvalue_2 _targetpoint) (Variables|Default|GetMinStopDistance) (Variables|Default|GetMaxDistanceDash))))
    (Ability|Tasks|ApplyRootMotionConstantForce "None" (Math|Vector|Normalize (- _targetpoint _returnvalue_2)) (Math|Float|Clamp(Float) (Math|Vector|Distance(Vector) _returnvalue_2 _targetpoint) (Variables|Default|GetMinStopDistance) (Variables|Default|GetMaxDistanceDash)) 0.1 false 0 "MaintainLastRootMotionVelocity"
      (:OnFinish
        (Ability|EndAbility)))
    (else
      (Ability|EndAbility))))

(event Ability|EventOnEndAbility
  (params (bWasCancelled :type Boolean))
  (GameplayEffects|RemoveActiveGameplayEffect (Ability|GetAbilitySystemComponent (Ability|GetAvatarActorfromActorInfo)) (Variables|Default|GetNewVar) -1))

(event Ability|EventActivateAbilityFromEvent
  (params (EventData :type Gameplay%20Event%20Data%20Structure%20%28by%20ref%29))
  (bind _returnvalue (Ability|GetAvatarActorfromActorInfo))
  (bind _returnvalue_2 (Transformation|GetActorLocation _returnvalue))
  (Development|PrintString (Utilities|String|ToString(Float) (Math|Float|Clamp(Float) (Math|Vector|Distance(Vector) _returnvalue_2 (stale Ability|EventActivateAbility _targetpoint)) (Variables|Default|GetMinStopDistance) (Variables|Default|GetMaxDistanceDash))))
  (Ability|Tasks|ApplyRootMotionConstantForce "None" (Math|Vector|Normalize (- (stale Ability|EventActivateAbility _targetpoint) _returnvalue_2)) (Math|Float|Clamp(Float) (Math|Vector|Distance(Vector) _returnvalue_2 (stale Ability|EventActivateAbility _targetpoint)) (Variables|Default|GetMinStopDistance) (Variables|Default|GetMaxDistanceDash)) 0.1 false 0 "MaintainLastRootMotionVelocity"
    (:OnFinish
      (Ability|EndAbility))))