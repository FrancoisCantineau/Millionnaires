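; Gameplay ability that dashes a BP_PsychistEnemy toward its current Target.
; On activation it commits, casts the avatar to the enemy and applies constant-force root motion along the normalized direction to the Target, then ends when the motion finishes.
; Event-triggered activation jumps straight to the dash, skipping commit and cast.
; Dash strength and duration are fixed; the distance-clamping nodes are unconnected.
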(event Ability|EventActivateAbility
  (Ability|CommitAbility)
  (bind _asbp_psychist_enemy (Utilities|Casting|CastToBP_PsychistEnemy (Ability|GetAvatarActorfromActorInfo)))
  (Ability|Tasks|ApplyRootMotionConstantForce "None" (Math|Vector|Normalize (- (Transformation|GetActorLocation (Variables|/Game/02_Blueprints/Ennemy/BP_PsychistEnemy.BP_PsychistEnemy_C|Gettarget _asbp_psychist_enemy)) (Transformation|GetActorLocation (Ability|GetAvatarActorfromActorInfo)))) 1e+03 0.3 false 0 "MaintainLastRootMotionVelocity"
    (:OnFinish
      (Ability|EndAbility))))

(event Ability|EventOnEndAbility
  (params (bWasCancelled :type Boolean)))

(event Ability|EventActivateAbilityFromEvent
  (params (EventData :type Gameplay%20Event%20Data%20Structure%20%28by%20ref%29))
  (Ability|Tasks|ApplyRootMotionConstantForce "None" (Math|Vector|Normalize (- (Transformation|GetActorLocation (Variables|/Game/02_Blueprints/Ennemy/BP_PsychistEnemy.BP_PsychistEnemy_C|Gettarget (stale Ability|EventActivateAbility _asbp_psychist_enemy))) (Transformation|GetActorLocation (Ability|GetAvatarActorfromActorInfo)))) 1e+03 0.3 false 0 "MaintainLastRootMotionVelocity"
    (:OnFinish
      (Ability|EndAbility))))