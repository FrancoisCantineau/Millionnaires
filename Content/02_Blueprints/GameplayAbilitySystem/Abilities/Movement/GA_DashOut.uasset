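; Gameplay ability that dashes an AI-controlled avatar toward the target point supplied by its AI controller.
; On activation it commits, applies GE_UsingAbility to the owner, then pushes the avatar with constant-force root motion for a fixed duration.
; The ability ends when the motion finishes or the commit fails, and ending removes the stored effect.
; Event-triggered activation jumps straight to the motion, skipping commit, effect and target lookup.
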(event Ability|EventActivateAbility
  (bind _returnvalue (Ability|CommitAbility))
  (if _returnvalue
    (bind _returnvalue_2 (Ability|ApplyGameplayEffectToOwner "/Game/02_Blueprints/GameplayAbilitySystem/Effects/GE_UsingAbility.GE_UsingAbility_C"))
    (Variables|Default|SetNewVar _returnvalue_2)
    (bind _targetpoint (Class|BPICombatInterface|GetTargetPoint(Message) (AI|GetAIController (Ability|GetAvatarActorfromActorInfo))))
    (Ability|Tasks|ApplyRootMotionConstantForce "None" (Math|Vector|Normalize (- _targetpoint (Transformation|GetActorLocation (Ability|GetAvatarActorfromActorInfo)))) 5e+02 0.5 false 0 "MaintainLastRootMotionVelocity"
      (:OnFinish
        (Ability|EndAbility)))
    (else
      (Ability|EndAbility))))

(event Ability|EventOnEndAbility
  (params (bWasCancelled :type Boolean))
  (GameplayEffects|RemoveActiveGameplayEffect (Ability|GetAbilitySystemComponent (Ability|GetAvatarActorfromActorInfo)) (Variables|Default|GetNewVar) -1))

(event Ability|EventActivateAbilityFromEvent
  (params (EventData :type Gameplay%20Event%20Data%20Structure%20%28by%20ref%29))
  (Ability|Tasks|ApplyRootMotionConstantForce "None" (Math|Vector|Normalize (- (stale Ability|EventActivateAbility _targetpoint) (Transformation|GetActorLocation (Ability|GetAvatarActorfromActorInfo)))) 5e+02 0.5 false 0 "MaintainLastRootMotionVelocity"
    (:OnFinish
      (Ability|EndAbility))))