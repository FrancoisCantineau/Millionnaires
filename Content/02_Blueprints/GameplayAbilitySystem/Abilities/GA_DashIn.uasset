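; GA_DashIn is a gameplay ability that dashes a BP_PsychistEnemy toward its Target.
; Standard activation commits the ability and caches the enemy avatar, while event-triggered activation skips both and joins the same dash logic.
; A very brief root motion constant force uses the clamped distance to the target as its strength and maintains velocity on finish, when the ability ends.
; Debug prints remain in the graph.
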(event Ability|EventActivateAbility
  (bind _returnvalue (Ability|GetAvatarActorfromActorInfo))
  (bind _returnvalue_2 (Transformation|GetActorLocation _returnvalue))
  (Ability|CommitAbility)
  (bind _asbp_psychist_enemy (Utilities|Casting|CastToBP_PsychistEnemy (Ability|GetAvatarActorfromActorInfo)))
  (Development|PrintString (Utilities|String|ToString(Float) (Math|Float|Clamp(Float) (Math|Vector|Distance(Vector) _returnvalue_2 (Transformation|GetActorLocation (Variables|/Game/02_Blueprints/Ennemy/BP_PsychistEnemy.BP_PsychistEnemy_C|Gettarget _asbp_psychist_enemy))) (Variables|Default|GetMinStopDistance) (Variables|Default|GetMaxDistanceDash))))
  (Ability|Tasks|ApplyRootMotionConstantForce "None" (Math|Vector|Normalize (- (Transformation|GetActorLocation (Variables|/Game/02_Blueprints/Ennemy/BP_PsychistEnemy.BP_PsychistEnemy_C|Gettarget _asbp_psychist_enemy)) _returnvalue_2)) (Math|Float|Clamp(Float) (Math|Vector|Distance(Vector) _returnvalue_2 (Transformation|GetActorLocation (Variables|/Game/02_Blueprints/Ennemy/BP_PsychistEnemy.BP_PsychistEnemy_C|Gettarget _asbp_psychist_enemy))) (Variables|Default|GetMinStopDistance) (Variables|Default|GetMaxDistanceDash)) 0.01 false 0 "MaintainLastRootMotionVelocity"
    (:OnFinish
      (Ability|EndAbility))))

(event Ability|EventOnEndAbility
  (params (bWasCancelled :type Boolean)))

(event Ability|EventActivateAbilityFromEvent
  (params (EventData :type Gameplay%20Event%20Data%20Structure%20%28by%20ref%29))
  (bind _returnvalue (Ability|GetAvatarActorfromActorInfo))
  (bind _returnvalue_2 (Transformation|GetActorLocation _returnvalue))
  (Development|PrintString "AAAAAAACTIVATion")
  (Development|PrintString (Utilities|String|ToString(Float) (Math|Float|Clamp(Float) (Math|Vector|Distance(Vector) _returnvalue_2 (Transformation|GetActorLocation (Variables|/Game/02_Blueprints/Ennemy/BP_PsychistEnemy.BP_PsychistEnemy_C|Gettarget (stale Ability|EventActivateAbility _asbp_psychist_enemy)))) (Variables|Default|GetMinStopDistance) (Variables|Default|GetMaxDistanceDash))))
  (Ability|Tasks|ApplyRootMotionConstantForce "None" (Math|Vector|Normalize (- (Transformation|GetActorLocation (Variables|/Game/02_Blueprints/Ennemy/BP_PsychistEnemy.BP_PsychistEnemy_C|Gettarget (stale Ability|EventActivateAbility _asbp_psychist_enemy))) _returnvalue_2)) (Math|Float|Clamp(Float) (Math|Vector|Distance(Vector) _returnvalue_2 (Transformation|GetActorLocation (Variables|/Game/02_Blueprints/Ennemy/BP_PsychistEnemy.BP_PsychistEnemy_C|Gettarget (stale Ability|EventActivateAbility _asbp_psychist_enemy)))) (Variables|Default|GetMinStopDistance) (Variables|Default|GetMaxDistanceDash)) 0.01 false 0 "MaintainLastRootMotionVelocity"
    (:OnFinish
      (Ability|EndAbility))))