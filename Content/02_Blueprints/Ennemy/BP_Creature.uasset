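; BP_Creature is a zombie enemy that grabs the player in a bite attack on overlapping its sphere.
; The overlap starts a paired contextual anim scene and an input challenge on the player controller.
; Challenge success or failure sets PushedCreature and switches both attacker and victim montages from Loop to the Exit or Bite section, respectively.
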(event OnComponentBeginOverlap(Sphere)
  (params (OverlappedComponent :type Primitive%20Component%20Object%20Reference) (OtherActor :type Actor%20Object%20Reference) (OtherComp :type Primitive%20Component%20Object%20Reference) (OtherBodyIndex :type Integer) (bFromSweep :type Boolean) (SweepResult :type Hit%20Result%20Structure%20%28by%20ref%29))
  (if (== OtherActor (Game|GetPlayerCharacter 0))
    (bind _outbindings (Class|ContextualAnimUtilities|CreateContextualAnimSceneBindingsforTwoActors "/Game/01-Arts/Meshes/Characters/Mannequins/Anims/ZombieAttack/CAS_ZombieBite.CAS_ZombieBite" (Class|ContextualAnimUtilities|SceneBindingContextMakefromActor self) (Class|ContextualAnimUtilities|SceneBindingContextMakefromActor OtherActor)))
    (Class|ContextualAnimSceneActorComponent|StartContextualAnimScene (Variables|Default|GetContextualAnimSceneActorComponent) _outbindings)
    (bind _asmillionnaires_player_controller (Utilities|Casting|CastToMillionnairesPlayerController (Game|GetPlayerController 0)))
    (Class|MillionnairesPlayerController|StartInputChallenge _asmillionnaires_player_controller "/Game/03-Game_Settings/Data/InteractAction/DA_ZombieBiteInteraction.DA_ZombieBiteInteraction")
    (EventDispatchers|BindEventtoOnSuccess (Actor|GetComponentbyClass _asmillionnaires_player_controller "/Script/InputChallenge.InputChallengeComponent") (delegate Custom|PushZombieAway))
    (EventDispatchers|BindEventtoOnFailure (Actor|GetComponentbyClass _asmillionnaires_player_controller "/Script/InputChallenge.InputChallengeComponent") (delegate Custom|CustomEvent))))

(event Custom|PushZombieAway
  (Variables|Default|SetbPushedCreature true)
  (Class|AnimInstance|MontageSetNextSection (Components|SkeletalMesh|GetAnimInstance (Variables|Character|GetMesh)) "Loop" "Exit" "/Game/CharacterCollection/Creature/Demo/Animations/AM_ZombieAttack_Attacker.AM_ZombieAttack_Attacker")
  (Class|AnimInstance|MontageSetNextSection (Components|SkeletalMesh|GetAnimInstance (Variables|/Script/Engine.Character|GetMesh (Game|GetPlayerCharacter 0))) "Loop" "Exit" "/Game/01-Arts/Meshes/Characters/Mannequins/Anims/ZombieAttack/AM_ZombieAttack_Victim.AM_ZombieAttack_Victim"))

(event Custom|CustomEvent
  (Variables|Default|SetbPushedCreature false)
  (Class|AnimInstance|MontageSetNextSection (Components|SkeletalMesh|GetAnimInstance (Variables|Character|GetMesh)) "Loop" "Bite" "/Game/CharacterCollection/Creature/Demo/Animations/AM_ZombieAttack_Attacker.AM_ZombieAttack_Attacker")
  (Class|AnimInstance|MontageSetNextSection (Components|SkeletalMesh|GetAnimInstance (Variables|/Script/Engine.Character|GetMesh (Game|GetPlayerCharacter 0))) "Loop" "Bite" "/Game/01-Arts/Meshes/Characters/Mannequins/Anims/ZombieAttack/AM_ZombieAttack_Victim.AM_ZombieAttack_Victim"))

(event EventBeginPlay
  (Variables|Default|Settarget (Game|Player|GetPlayerPawn 0)))

(fn ConstructionScript)