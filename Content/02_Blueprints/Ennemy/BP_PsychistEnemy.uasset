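; BP_PsychistEnemy is a Psychist enemy Blueprint whose only live logic sets its Target to the player pawn on BeginPlay.
; Tick and the construction script are empty.
; Disconnected nodes hold unused Gameplay Ability System experiments: granting abilities, triggering best or random Psy-tagged abilities on the player through AbilityHandler, and printing attribute values.
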(event EventBeginPlay
  (Variables|Default|Settarget (Game|Player|GetPlayerPawn 0)))

(event EventTick
  (params (DeltaSeconds :type Float%20%28single-precision%29)))

(fn ConstructionScript)