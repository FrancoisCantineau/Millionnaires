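; BP_LightInvisibleEnemy is an enemy that is visible only when lit.
; Its LightAwareness component reports light intensity, and the Blueprint switches the mesh material's Visibility parameter fully on or off around a low threshold.
; Separately, a Sphere trigger sends a Flicker message to actors entering or leaving it, turning their flicker on and off.
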(event OnComponentBeginOverlap(Sphere)
  (params (OverlappedComponent :type Primitive%20Component%20Object%20Reference) (OtherActor :type Actor%20Object%20Reference) (OtherComp :type Primitive%20Component%20Object%20Reference) (OtherBodyIndex :type Integer) (bFromSweep :type Boolean) (SweepResult :type Hit%20Result%20Structure%20%28by%20ref%29))
  (Class|Lights|Flicker(Message) OtherActor true))

(event OnComponentEndOverlap(Sphere)
  (params (OverlappedComponent :type Primitive%20Component%20Object%20Reference) (OtherActor :type Actor%20Object%20Reference) (OtherComp :type Primitive%20Component%20Object%20Reference) (OtherBodyIndex :type Integer))
  (Class|Lights|Flicker(Message) OtherActor false))

(event Custom|LightIntensity
  (params (CurrentLightValue :type Float%20%28single-precision%29))
  (if (<= CurrentLightValue 0.2)
    (Rendering|Material|SetScalarParameterValueonMaterials (Variables|Character|GetMesh) "Visibility" 0.0)
    (else
      (Rendering|Material|SetScalarParameterValueonMaterials (Variables|Character|GetMesh) "Visibility" 1.0))))

(event EventBeginPlay
  (|CallParentFunction)
  (EventDispatchers|BindEventtoOnLightAwarenessComponentUpdated (Variables|Default|GetLightAwareness) (delegate Custom|LightIntensity))
  (Rendering|Material|CreateDynamicMaterialInstance (Variables|Character|GetMesh) 0 "/Game/01-Arts/Meshes/Characters/Mannequins/Materials/M_MannequinInvisible.M_MannequinInvisible" "None" :!class /Script/Engine.PrimitiveComponent)
  (Variables|Default|Settarget (Game|Player|GetPlayerPawn 0)))

(fn ConstructionScript)