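; BP_Elevator is a procedural-map elevator that moves its mesh toward a registered floor when a Pawn enters its box.
; AddNewFloor fills a map of floors, though the trip always targets the entry at index 0.
; A Timeline lerps from the mesh's location at overlap to that floor's SMElevator location.
; On finish it sets the current floor to 1, calls NewFloorReached and prints a debug string.
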(event OnComponentBeginOverlap(Box)
  (params (OverlappedComponent :type Primitive%20Component%20Object%20Reference) (OtherActor :type Actor%20Object%20Reference) (OtherComp :type Primitive%20Component%20Object%20Reference) (OtherBodyIndex :type Integer) (bFromSweep :type Boolean) (SweepResult :type Hit%20Result%20Structure%20%28by%20ref%29))
  (bind _sm_elevator (Variables|Default|GetSM_Elevator))
  (Utilities|Casting|CastToPawn OtherActor)
  (Variables|Default|SetNewVar (Transformation|GetWorldLocation _sm_elevator))
  (bind _newtrack_0 (Timeline|Timeline Play)
    (:Update
      (Transformation|SetWorldLocation _sm_elevator (Math|Vector|Lerp(Vector) (Variables|Default|GetNewVar) (Transformation|GetWorldLocation (Variables|BP_Elevator_C|GetSM_Elevator (.Value (Utilities|Map|GetKeyValueByIndex (Variables|Default|GetFloor/Elevator) 0)))) _newtrack_0) false false))
    (:Finished
      (bind _output_get (Variables|Default|SetCurrentFloorPosition 1))
      (Default|CallNewFloorReached _output_get)
      (Development|PrintString "Hello"))))

(event Custom|AddNewFloor
  (params (NewFloor :type BP%20Elevator%20Object%20Reference) (Floor :type Integer))
  (Utilities|Map|Add (Variables|Default|GetFloor/Elevator) Floor NewFloor))

(event EventBeginPlay)

(event Collision|EventActorBeginOverlap
  (params (OtherActor :type Actor%20Object%20Reference)))

(event EventTick
  (params (DeltaSeconds :type Float%20%28single-precision%29)))

(fn ConstructionScript)