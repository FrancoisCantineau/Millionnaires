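; Base room actor for procedural factory map generation, which registers the room's connection points.
; On BeginPlay it gathers the direct children of the Connexions0 component into ConexionsArray0 without duplicates.
; A nested pass over the same children casts child actor components to DoorArrow actors and stores them uniquely in DoorsArray0.
; Tick and the construction script are empty, so any map assembly logic lives outside these graphs.
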(event EventBeginPlay
  (for _array_element (Components|GetChildrenComponents (Variables|Default|GetConnexions_0) false)
    (Utilities|Array|AddUnique (Variables|Default|GetConexionsArray_0) _array_element)
    (for _array_element_2 (Components|GetChildrenComponents (Variables|Default|GetConnexions_0) false)
      (bind _aschild_actor_component (Utilities|Casting|CastToChildActorComponent _array_element_2))
      (bind _asdoor_arrow (Utilities|Casting|CastToDoorArrow (Variables|/Script/Engine.ChildActorComponent|GetChildActor _aschild_actor_component)))
      (Utilities|Array|AddUnique (Variables|Default|GetDoorsArray_0) _asdoor_arrow))))

(event EventTick
  (params (DeltaSeconds :type Float%20%28single-precision%29)))

(fn ConstructionScript)