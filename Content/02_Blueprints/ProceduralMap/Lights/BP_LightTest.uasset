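; BP_LightTest is a test light actor for the procedural map that stores the zone type it is initialized with.
; On BeginPlay it caches the first child of LightComp as its light component, then runs the parent BeginPlay after a short delay, stopping if the cast fails.
; FlickerResult supplies a random on/off flicker value, weighted toward off, but nothing in this Blueprint calls it.
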(event Custom|Initialize
  (params (ZoneType :type Gameplay%20Tag%20Structure))
  (Variables|Default|SetZoneType ZoneType))

(event EventBeginPlay
  (bind _aslight_component (Utilities|Casting|CastToLightComponent (Components|GetChildComponent (Variables|Default|GetLightComp) 0)))
  (Variables|Default|SetLightComponent _aslight_component)
  (Utilities|FlowControl|Delay 1.0)
  (|CallParentFunction))

(fn ConstructionScript)

(fn FlickerResult
  (return (Math|Float|SelectFloat 1.0 0.0 (> (Math|Random|RandomFloatinRange 0.0 1.0) 0.7))))