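; LED strip light actor for the procedural map that reacts to power failure and restoration from ship incidents tagged as affecting lights.
; Power failure applies configured emergency color and intensity, with optional rotation and timeline-driven pulsing of light and emissive material.
; Flicker uses a looping timer with random on/off results to drive light-function and emissive parameters, plus sparks and sound.
; Restore stops the pulse, but PowerLight currently zeroes spotlight intensity either way.
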(event Custom|FlickerEvent
  (bind _niagara_config (Variables|Default|GetNiagara%20Config))
  (bind (_bsparkenabled _sparksystem) (Utilities|Struct|BreakLampNiagaraConfig _niagara_config))
  (bind _flickeringvalue (CallFunction|FlickerResult))
  (if (>= _flickeringvalue 1.0)
    (if (Variables|Flickering|GetLastState)
      (Rendering|Material|SetScalarParameterValue (Variables|Flickering|GetFlickeringDynamicMaterial) "Intensity" _flickeringvalue :!class /Script/Engine.MaterialInstanceDynamic :!label _label)
      (Rendering|Material|SetScalarParameterValue (Variables|Default|GetMaterialInstance) "EmissionMultiplicator" _flickeringvalue :!class /Script/Engine.MaterialInstanceDynamic)
      (else
        (Variables|Flickering|SetLastState true)
        (if (Utilities|IsValidSoftObjectReference (Utilities|ResolveSoftReference (Utilities|Struct|BreakLampSoundConfig (Variables|Default|GetSoundConfig))))
          (Audio|PlaySoundatLocation 0 (Transformation|GetActorLocation) "0, 0, 0" 1.0 1.0 0.0 "/Game/UltraDynamicSky/Sound/Attenuation/UDS_Interact_Sound_Attenuation.UDS_Interact_Sound_Attenuation" 0 0 0)
          (goto _label))))
    (elif (Variables|Flickering|GetLastState)
      (if (and _bsparkenabled (Utilities|IsValidSoftObjectReference (Utilities|ResolveSoftReference _sparksystem)))
        (Components|Activation|Activate (Variables|Default|GetSparks) true)
        (Variables|Flickering|SetLastState false))
      (if true
        (goto _label)
        (else
          (goto _label)))
      (else
        (goto _label)))))

(event Custom|IncidentTriggered
  (params (Incident :type Ship%20Incident%20Structure))
  (if (GameplayTags|HasTag (Utilities|Struct|BreakShipIncident Incident) "(TagName=\"Incident.AffectsSystem.Light\")")
    (Class|LightBase|OnPowerFailure)))

(event Custom|IncidentResolved
  (params (Incident :type Ship%20Incident%20Structure))
  (if (GameplayTags|HasTag (Utilities|Struct|BreakShipIncident Incident) "(TagName=\"Incident.AffectsSystem.Light\")")
    (Class|LightBase|OnPowerRestore)))

(event EventBeginPlay
  (bind _aslight_component (Utilities|Casting|CastToLightComponent (Components|GetChildComponent (Variables|Default|GetLightComp) 0)))
  (Variables|Default|SetLightComponent _aslight_component)
  (Utilities|FlowControl|Delay 1.0)
  (|CallParentFunction))

(event Collision|EventActorBeginOverlap
  (params (OtherActor :type Actor%20Object%20Reference)))

(event EventOnPowerFailure
  (bind _returnvalue (Class|LightBase|GetActiveConfig))
  (bind _rotatingmovement (Variables|Default|GetRotatingMovement))
  (bind _spotlight (Variables|Default|GetSpotLight))
  (bind (_breactstopowerfailure _bisemergencylight _emergencycolor _emergencyintensity _bshouldpulse _pulsespeed _pulseminintensityratio _pulsemaxintensityratio _bisrotatinglight) (Utilities|Struct|BreakEmergencyLightConfig (.emergencysettings _returnvalue)))
  (if true
    (if _bisrotatinglight
      (Variables|/Script/Engine.RotatingMovementComponent|SetRotationRate _rotatingmovement (Math|Rotator|MakeRotator 0.0 0.0 1.8e+02))
      (Components|Activation|Activate _rotatingmovement false))
    (Rendering|Components|Light|SetLightColor _spotlight _emergencycolor true)
    (Rendering|Components|Light|SetIntensity _spotlight _emergencyintensity)
    (if _bshouldpulse
      (Components|Timeline|SetPlayRate (Variables|Default|GetPulseTimeline) _pulsespeed)
      (bind _pulse (Timeline|PulseTimeline Play)
        (:Update
          (Rendering|Components|Light|SetIntensity (Variables|Default|GetSpotLight) (Math|Float|Lerp (* _pulseminintensityratio _emergencyintensity) (* _pulsemaxintensityratio _emergencyintensity) _pulse))
          (Rendering|Material|SetScalarParameterValue (Variables|Default|GetMaterialInstance) "EmissionMultiplicator" _pulse :!class /Script/Engine.MaterialInstanceDynamic)))
      (else
        (Rendering|Material|SetScalarParameterValue (Variables|Default|GetMaterialInstance) "EmissionMultiplicator" 0.0 :!class /Script/Engine.MaterialInstanceDynamic)))
    (else
      (Rendering|Material|SetScalarParameterValue (Variables|Default|GetMaterialInstance) "EmissionMultiplicator" 0.0 :!class /Script/Engine.MaterialInstanceDynamic)
      (Rendering|Components|Light|SetIntensity (Variables|Default|GetSpotLight) 0.0))))

(event EventFlicker
  (params (bShouldFlicker :type Boolean))
  (if bShouldFlicker
    (Utilities|FlowControl|Sequence
      (:then_0
        (Utilities|FlowControl|DoOnce false
          (:Completed
            (bind _returnvalue (Rendering|Material|CreateDynamicMaterialInstance "/Game/01-Arts/Materials/M_FlickeringLight.M_FlickeringLight" "None" "None" :!class /Script/Engine.KismetMaterialLibrary))
            (Variables|Flickering|SetFlickeringDynamicMaterial _returnvalue))))
      (:then_1
        (Rendering|Components|Light|SetLightFunctionMaterial (Variables|Default|GetSpotLight) (Variables|Flickering|GetFlickeringDynamicMaterial))
        (bind _returnvalue_2 (Utilities|Time|SetTimerbyEvent (delegate Custom|FlickerEvent) 0.0 true true))
        (Variables|Flickering|SetFlickeringTimer _returnvalue_2)))
    (else
      (Rendering|Components|Light|SetLightFunctionMaterial (Variables|Default|GetSpotLight) 0)
      (Utilities|Time|ClearandInvalidateTimerbyHandle (Variables|Flickering|GetFlickeringTimer)))))

(event EventFlickerLight
  (if true
    (Utilities|FlowControl|Sequence
      (:then_0
        (Utilities|FlowControl|DoOnce false
          (:Completed
            (bind _returnvalue (Rendering|Material|CreateDynamicMaterialInstance "/Game/01-Arts/Materials/M_FlickeringLight.M_FlickeringLight" "None" "None" :!class /Script/Engine.KismetMaterialLibrary))
            (Variables|Flickering|SetFlickeringDynamicMaterial _returnvalue))))
      (:then_1
        (Rendering|Components|Light|SetLightFunctionMaterial (Variables|Default|GetSpotLight) (Variables|Flickering|GetFlickeringDynamicMaterial))
        (bind _returnvalue_2 (Utilities|Time|SetTimerbyEvent (delegate Custom|FlickerEvent) 0.0 true true))
        (Variables|Flickering|SetFlickeringTimer _returnvalue_2)))))

(event EventPowerLight
  (params (bShouldPower :type Boolean))
  (bind _ambiancesound (Variables|Default|GetAmbianceSound))
  (if bShouldPower
    (Rendering|Components|Light|SetIntensity (Variables|Default|GetSpotLight) 0.0)
    (Rendering|Components|Light|SetLightColor :self (Variables|Default|GetSpotLight))
    (Audio|Components|Audio|SetSound _ambiancesound 0)
    (Audio|Components|Audio|Play _ambiancesound 0.0)
    (Rendering|Material|SetScalarParameterValue (Variables|Default|GetMaterialInstance) "EmissionMultiplicator" 1.0 :!class /Script/Engine.MaterialInstanceDynamic)
    (else
      (Audio|Components|Audio|Stop (Variables|Default|GetAmbianceSound))
      (Rendering|Components|Light|SetIntensity (Variables|Default|GetSpotLight) 0.0))))

(event EventOnPowerRestore
  (bind _returnvalue (Class|LightBase|GetActiveConfig))
  (bind (_breactstopowerfailure _bisemergencylight _emergencycolor _emergencyintensity _bshouldpulse _pulsespeed _pulseminintensityratio _pulsemaxintensityratio _bisrotatinglight) (Utilities|Struct|BreakEmergencyLightConfig (.emergencysettings _returnvalue)))
  (Class|LightBase|PowerLight true)
  (bind _pulse (Timeline|PulseTimeline Stop)
    (:Update
      (Rendering|Components|Light|SetIntensity (Variables|Default|GetSpotLight) (Math|Float|Lerp (* _pulseminintensityratio _emergencyintensity) (* _pulsemaxintensityratio _emergencyintensity) _pulse))
      (Rendering|Material|SetScalarParameterValue (Variables|Default|GetMaterialInstance) "EmissionMultiplicator" _pulse :!class /Script/Engine.MaterialInstanceDynamic))))

(fn ConstructionScript)

(fn FlickerResult
  (return (Math|Float|SelectFloat 1.0 0.0 (> (Math|Random|RandomFloatinRange 0.0 1.0) 0.7))))