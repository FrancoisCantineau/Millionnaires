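; Test actor for a procedural-map light that flickers and reacts to incidents, self-triggering a Fire incident in its zone on BeginPlay and resolving it after a delay.
; A looping timer randomly switches a light-function material and mesh emissive together until any incident stops it.
; Incidents affecting lights cut power or start config-driven emergency lighting with optional rotation and timeline pulse.
; Their resolution restores configured intensity, color and ambient sound.
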(event Custom|FlickerEvent
  (bind _flickeringvalue (CallFunction|FlickerResult))
  (if (>= _flickeringvalue 1.0)
    (if (Variables|Flickering|GetLastState)
      _
      (else
        (Variables|Flickering|SetLastState true)))
    (elif (Variables|Flickering|GetLastState)
      (Variables|Flickering|SetLastState false)))
  (Rendering|Material|SetScalarParameterValue (Variables|Flickering|GetFlickeringDynamicMaterial) "Intensity" _flickeringvalue :!class /Script/Engine.MaterialInstanceDynamic)
  (Rendering|Material|SetScalarParameterValue (Variables|Default|GetMaterialInstance) "EmissionMultiplicator" _flickeringvalue :!class /Script/Engine.MaterialInstanceDynamic))

(event Custom|CustomEvent
  (params (Incident :type Ship%20Incident%20Structure))
  (CallFunction|Flicker false)
  (if (GameplayTags|HasTag (.AffectedSystems (Utilities|Struct|BreakShipIncident Incident)) "(TagName=\"Incident.AffectsSystem.Light\")")
    (Development|PrintString "Hello")
    (Class|LightBase|OnPowerFailure)
    (else
      (Development|PrintString "Hello"))))

(event Custom|CustomEvent_0
  (params (Incident :type Ship%20Incident%20Structure))
  (if (GameplayTags|HasTag (.AffectedSystems (Utilities|Struct|BreakShipIncident Incident)) "(TagName=\"Incident.AffectsSystem.Light\")")
    (Class|LightBase|OnPowerRestore)))

(event EventBeginPlay
  (bind _returnvalue (Subsystems|GetIncidentManager))
  (bind _returnvalue_2 (Subsystems|GetIncidentManager))
  (bind _sm_light_f (Variables|Default|GetSM_Light_F))
  (bind _returnvalue_3 (Rendering|Material|CreateDynamicMaterialInstance _sm_light_f 0 (Rendering|Material|GetMaterial _sm_light_f 0) "None" :!class /Script/Engine.PrimitiveComponent))
  (Variables|Default|SetMaterialInstance _returnvalue_3)
  (Class|LightBase|FlickerLight)
  (EventDispatchers|BindEventtoOnIncidentTriggered _returnvalue_2 (delegate Custom|CustomEvent))
  (bind _returnvalue_4 (Class|IncidentManager|TriggerIncident _returnvalue_2 (Utilities|Struct|MakeShipIncident "(TagName=\"Incident.Fire\")" "(TagName=\"Zone\")" 0 false 0.0 "(GameplayTags=((TagName=\"Incident.AffectsSystem.Door\"),(TagName=\"Incident.AffectsSystem.Light\")))")))
  (EventDispatchers|BindEventtoOnIncidentResolved _returnvalue (delegate Custom|CustomEvent_0))
  (Utilities|FlowControl|Delay 1e+01)
  (Class|IncidentManager|ResolveIncident _returnvalue _returnvalue_4))

(event Collision|EventActorBeginOverlap
  (params (OtherActor :type Actor%20Object%20Reference)))

(event EventOnPowerFailure
  (bind _returnvalue (Class|LightBase|GetActiveConfig))
  (bind _rotatingmovement (Variables|Default|GetRotatingMovement))
  (bind _spotlight (Variables|Default|GetSpotLight))
  (bind (_emergencycolor _emergencyintensity _bshouldpulse _pulsespeed _pulseminintensityratio _pulsemaxintensityratio _bisrotatinglight) (Utilities|Struct|BreakEmergencyLightConfig (.emergencysettings _returnvalue)))
  (if (.bIsEmergencyLight (Utilities|Struct|BreakLampPowerConfig (.power _returnvalue)))
    (if _bisrotatinglight
      (Variables|/Script/Engine.RotatingMovementComponent|SetRotationRate _rotatingmovement (Math|Rotator|MakeRotator 0.0 0.0 1.8e+02))
      (Components|Activation|Activate _rotatingmovement false))
    (Rendering|Components|Light|SetLightColor _spotlight _emergencycolor true)
    (Rendering|Components|Light|SetIntensity _spotlight _emergencyintensity)
    (if _bshouldpulse
      (Components|Timeline|SetPlayRate (Variables|Default|GetPulseTimeline) _pulsespeed)
      (bind _pulse (Timeline|PulseTimeline Play)
        (:Update
          (Rendering|Components|Light|SetIntensity (Variables|Default|GetSpotLight) (Math|Float|Lerp (* _pulseminintensityratio _emergencyintensity) (* _pulsemaxintensityratio _emergencyintensity) _pulse))
          (Rendering|Material|SetScalarParameterValue (Variables|Default|GetMaterialInstance) "EmissionMultiplicator" _pulse :!class /Script/Engine.MaterialInstanceDynamic)))
      (else
        (Rendering|Material|SetScalarParameterValue (Variables|Default|GetMaterialInstance) "EmissionMultiplicator" 0.0 :!class /Script/Engine.MaterialInstanceDynamic)))
    (else
      (Rendering|Material|SetScalarParameterValue (Variables|Default|GetMaterialInstance) "EmissionMultiplicator" 0.0 :!class /Script/Engine.MaterialInstanceDynamic)
      (Rendering|Components|Light|SetIntensity (Variables|Default|GetSpotLight) 0.0))))

(event EventFlicker
  (params (bShouldFlicker :type Boolean))
  (if bShouldFlicker
    (Utilities|FlowControl|Sequence
      (:then_0
        (Utilities|FlowControl|DoOnce false
          (:Completed
            (bind _returnvalue (Rendering|Material|CreateDynamicMaterialInstance "/Game/01-Arts/Materials/M_FlickeringLight.M_FlickeringLight" "None" "None" :!class /Script/Engine.KismetMaterialLibrary))
            (Variables|Flickering|SetFlickeringDynamicMaterial _returnvalue))))
      (:then_1
        (Rendering|Components|Light|SetLightFunctionMaterial (Variables|Default|GetSpotLight) (Variables|Flickering|GetFlickeringDynamicMaterial))
        (bind _returnvalue_2 (Utilities|Time|SetTimerbyEvent (delegate Custom|FlickerEvent) 0.8 true true))
        (Variables|Flickering|SetFlickeringTimer _returnvalue_2)))
    (else
      (Rendering|Components|Light|SetLightFunctionMaterial (Variables|Default|GetSpotLight) 0)
      (Utilities|Time|ClearandInvalidateTimerbyHandle (Variables|Flickering|GetFlickeringTimer)))))

(event EventFlickerLight
  (Utilities|FlowControl|Sequence
    (:then_0
      (Utilities|FlowControl|DoOnce false
        (:Completed
          (bind _returnvalue (Rendering|Material|CreateDynamicMaterialInstance "/Game/01-Arts/Materials/M_FlickeringLight.M_FlickeringLight" "None" "None" :!class /Script/Engine.KismetMaterialLibrary))
          (Variables|Flickering|SetFlickeringDynamicMaterial _returnvalue))))
    (:then_1
      (Rendering|Components|Light|SetLightFunctionMaterial (Variables|Default|GetSpotLight) (Variables|Flickering|GetFlickeringDynamicMaterial))
      (bind _returnvalue_2 (Utilities|Time|SetTimerbyEvent (delegate Custom|FlickerEvent) 0.8 true true))
      (Variables|Flickering|SetFlickeringTimer _returnvalue_2))))

(event EventPowerLight
  (params (bShouldPower :type Boolean))
  (bind _returnvalue (Class|LightBase|GetActiveConfig))
  (bind _ambiancesound (Variables|Default|GetAmbianceSound))
  (bind (_intensity _color) (Utilities|Struct|BreakLampLightConfig (.light _returnvalue)))
  (if bShouldPower
    (Rendering|Components|Light|SetIntensity (Variables|Default|GetSpotLight) _intensity)
    (Rendering|Components|Light|SetLightColor (Variables|Default|GetSpotLight) _color true)
    (Audio|Components|Audio|SetSound _ambiancesound (Utilities|ResolveSoftReference (.AmbientSound (Utilities|Struct|BreakLampSoundConfig (.sound _returnvalue)))))
    (Audio|Components|Audio|Play _ambiancesound 0.0)
    (Rendering|Material|SetScalarParameterValue (Variables|Default|GetMaterialInstance) "EmissionMultiplicator" 1.0 :!class /Script/Engine.MaterialInstanceDynamic)
    (else
      (Audio|Components|Audio|Stop (Variables|Default|GetAmbianceSound))
      (Rendering|Components|Light|SetIntensity (Variables|Default|GetSpotLight) 0.0))))

(event EventOnPowerRestore
  (bind _returnvalue (Class|LightBase|GetActiveConfig))
  (bind (_emergencycolor _emergencyintensity _bshouldpulse _pulsespeed _pulseminintensityratio _pulsemaxintensityratio _bisrotatinglight) (Utilities|Struct|BreakEmergencyLightConfig (.emergencysettings _returnvalue)))
  (Class|LightBase|PowerLight true)
  (bind _pulse (Timeline|PulseTimeline Stop)
    (:Update
      (Rendering|Components|Light|SetIntensity (Variables|Default|GetSpotLight) (Math|Float|Lerp (* _pulseminintensityratio _emergencyintensity) (* _pulsemaxintensityratio _emergencyintensity) _pulse))
      (Rendering|Material|SetScalarParameterValue (Variables|Default|GetMaterialInstance) "EmissionMultiplicator" _pulse :!class /Script/Engine.MaterialInstanceDynamic))))

(fn ConstructionScript)

(fn FlickerResult
  (return (Math|Float|SelectFloat 1.0 0.0 (> (Math|Random|RandomFloatinRange 0.0 1.0) 0.7))))