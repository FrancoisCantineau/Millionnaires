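; Procedural map generator that builds a level at BeginPlay from weighted room modules, with per-floor caps per room type.
; It snaps random room doors onto open connections, rejects overlapping placements, caps connections when no module fits, and restarts if none remain open.
; Saved room data feeds a 3D map build, then elevator rooms seed another floor below.
; Shortcut creation is an empty stub, with its spline-linking logic left disconnected.
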(event Custom|SpawnNextRoom
  ;[0.15 0.1165 0.04275 0.5] Spawns a room
  (Variables|Default|GetCurentlyTestedFreeConnexion
    (:then
      (bind _spawnblocked_ (CallFunction|SpawnRoom&Test :!label _label))
      (if _spawnblocked_
        (Utilities|Array|RemoveItem (Variables|Default|GetCurrentTestedModules) (Variables|Default|GetCurrentlyTestedRoom))
        (if (Utilities|Array|IsEmpty (Variables|Default|GetCurrentTestedModules))
          (Utilities|Array|RemoveItem (Variables|Default|GetFreeConnexionsList) (Variables|Default|GetCurentlyTestedFreeConnexion))
          (Utilities|Array|Clear (Variables|Default|GetCurrentTestedModules))
          (for _array_element (Variables|Default|GetFloorValidModules)
            (Utilities|Array|AddUnique (Variables|Default|GetCurrentTestedModules) _array_element))
          (CallFunction|CloseDoor (Variables|Default|GetCurentlyTestedFreeConnexion))
          (Variables|Default|SetCurentlyTestedFreeConnexion 0)
          (CallFunction|SpawnNextRoom)
          (else
            (CallFunction|SpawnNextRoom)))
        (else
          (CallFunction|SaveRoomData)
          (CallFunction|ModifyCurrentRoom/Floor)
          (Utilities|Array|Clear (Variables|Default|GetCurrentTestedModules))
          (for _array_element_2 (Variables|Default|GetFloorValidModules)
            (Utilities|Array|AddUnique (Variables|Default|GetCurrentTestedModules) _array_element_2))
          (Utilities|Array|AppendArray (Variables|Default|GetFreeConnexionsList) (Variables|/Game/02_Blueprints/ProceduralMap/BP_Room_Base.BP_Room_Base_C|GetConexionsArray (Variables|Default|GetCurrentRoom)))
          (Utilities|Array|RemoveItem (Variables|Default|GetFreeConnexionsList) (Variables|Default|GetCurentlyTestedFreeConnexion))
          (Utilities|Array|RemoveItem (Variables|Default|GetFreeConnexionsList) (Variables|Default|GetCurrentNewRoomDoor))
          (Utilities|Array|AddUnique (Variables|Default|GetSpawnedRooms) (Variables|Default|GetCurrentRoom))
          (Variables|Default|SetCurentlyTestedFreeConnexion 0)
          (Math|Integer|IncrementInt (Variables|Default|GetCurrentRoomSpawnIndex)
            (:%20%20
              (if (> (Variables|Default|GetMaxModules) (Variables|Default|GetCurrentRoomSpawnIndex))
                (Utilities|FlowControl|Delay 0.0)
                (CallFunction|SpawnNextRoom)
                (else
                  (CallFunction|CreateShortcut)
                  (Default|Build3DMap (Variables|Default|Get3dMap) (Variables|Default|GetSavedRoomData))
                  (CallFunction|SetupNextFloor))))))))
    (:else
      (bind _output_get (Variables|Default|SetCurentlyTestedFreeConnexion (.OutItem (Utilities|Array|Random (Variables|Default|GetFreeConnexionsList)))))
      (Utilities|IsValid _output_get
        (:Is%20Valid
          (goto _label))
        (:Is%20Not%20Valid
          (CallFunction|RestartGeneration))))))

(event Custom|CreateShortcut)

(event Custom|RestartGeneration
  (for _array_element (Variables|Default|GetSpawnedRooms)
    (Actor|DestroyActor _array_element))
  (Utilities|Array|Clear (Variables|Default|GetSavedRoomData))
  (for _array_element_2 (Variables|Default|GetPossibleModules)
    (Utilities|Map|Clear (.FloorCurrentRoomAmount (Utilities|Struct|BreakS_RoomStruct _array_element_2))))
  (Utilities|FlowControl|DelayUntilNextFrame)
  (CallFunction|StartGeneration))

(event Custom|StartGeneration
  ;[0.15 0.01276 0.01276 0.5] Instantiate first room and launch next steps
  (bind _returnvalue (Game|SpawnActorfromClass (Variables|Default|GetFirstRoom) (Math|Transform|MakeTransform "0, 0, 0" "0, 0, 0" "1.000000,1.000000,1.000000") "Undefined" "MultiplyWithRoot" 0 0))
  (CallFunction|SetupArray/Variables)
  (Utilities|Array|AppendArray (Variables|Default|GetFreeConnexionsList) (Variables|/Game/02_Blueprints/ProceduralMap/BP_Room_Base.BP_Room_Base_C|GetConexionsArray _returnvalue))
  (CallFunction|SpawnNextRoom))

(event Custom|SetupNextFloor
  (Math|Integer|IncrementInt (Variables|Default|GetCurrentFloor)
    (:%20%20
      (if (< (Variables|Default|GetCurrentFloor) 2)
        (for _array_element (Variables|Default|GetSpawnedRooms)
          (if (Utilities|Enum|Equal(Enum) (Variables|/Game/02_Blueprints/ProceduralMap/BP_Room_Base.BP_Room_Base_C|GetRoomType _array_element) "NewEnumerator3")
            (bind _returnvalue (Game|SpawnActorfromClass "/Game/02_Blueprints/ProceduralMap/BP_Elevator.BP_Elevator_C" (Math|Transform|MakeTransform (Math|Vector|MakeVector (.x (.Location (Math|Transform|BreakTransform (.Position (Utilities|Struct|BreakS_RoomData (stale _array_element)))))) (.y (.Location (Math|Transform|BreakTransform (.Position (Utilities|Struct|BreakS_RoomData (stale _array_element)))))) (- (.z (.Location (Math|Transform|BreakTransform (.Position (Utilities|Struct|BreakS_RoomData (stale _array_element)))))) 3e+03)) (.Rotation (Math|Transform|BreakTransform (.Position (Utilities|Struct|BreakS_RoomData (stale _array_element))))) (.Scale (Math|Transform|BreakTransform (.Position (Utilities|Struct|BreakS_RoomData (stale _array_element)))))) "AlwaysSpawn" "MultiplyWithRoot" 0 0))
            (bind _asbp_elevator (Utilities|Casting|CastToBP_Elevator _array_element))
            (Default|AddNewFloor _asbp_elevator _returnvalue (Variables|Default|GetCurrentFloor))
            (CallFunction|SetupArray/Variables)
            (Utilities|Array|AppendArray (Variables|Default|GetFreeConnexionsList) (Variables|/Game/02_Blueprints/ProceduralMap/BP_Room_Base.BP_Room_Base_C|GetConexionsArray _returnvalue))
            (CallFunction|SpawnNextRoom)))))))

(event Custom|SetupArray/Variables
  ;[0.0129 0.15 0.1342 0.5] Setup cariables/array for the generation
  (Utilities|Array|Clear (Variables|Default|GetFreeConnexionsList))
  (Variables|Default|SetCurrentRoomSpawnIndex 0)
  (Variables|Default|SetCurrentNewRoomDoor 0)
  (Variables|Default|SetCurentlyTestedFreeConnexion 0)
  (Variables|Default|SetCurrentRoom 0)
  (Utilities|Array|Clear (Variables|Default|GetFloorValidModules))
  (Utilities|Array|AppendArray (Variables|Default|GetFloorValidModules) (Variables|Default|GetPossibleModules))
  (Utilities|Array|Clear (Variables|Default|GetCurrentTestedModules))
  (for _array_element (Variables|Default|GetFloorValidModules)
    (Utilities|Array|AddUnique (Variables|Default|GetCurrentTestedModules) _array_element)))

(event EventBeginPlay
  (CallFunction|StartGeneration))

(fn ConstructionScript)

(fn CheckOverlap
  (bind _overlappingarray (Variables|Default|GetOverlappingArray))
  (for _array_element (Components|GetChildrenComponents (Variables|/Game/02_Blueprints/ProceduralMap/BP_Room_Base.BP_Room_Base_C|GetOverlappingComp (Variables|Default|GetCurrentRoom)) false)
    (bind _asbox_collision (Utilities|Casting|CastToBoxComponent _array_element))
    (Utilities|Array|AppendArray (Variables|Default|GetOverlappingArray) (Class|PrimitiveComponent|GetOverlappingComponents _asbox_collision)))
  (if (Utilities|Array|IsEmpty _overlappingarray)
    (return false)
    (else
      (Utilities|Array|Clear _overlappingarray)
      (Actor|DestroyActor (Variables|Default|GetCurrentRoom))
      (Variables|Default|SetCurrentRoom 0)
      (return true))))

(fn SpawnRoom&Test
  ;[0.15 0.09913 0 0.5] SpawnNextRoom
  (bind _randomfound (CallFunction|FindARandomWeighted))
  (if _randomfound
    (bind _returnvalue (Game|SpawnActorfromClass (.RoomClass (Utilities|Struct|BreakS_RoomStruct (Variables|Default|GetCurrentlyTestedRoom))) (Transformation|GetWorldTransform (Variables|Default|GetCurentlyTestedFreeConnexion)) "AlwaysSpawn" "MultiplyWithRoot" 0 0))
    (bind _output_get (Variables|Default|SetCurrentRoom _returnvalue))
    (Variables|Default|SetCurrentNewRoomDoor (Utilities|Array|Get(acopy) (Variables|/Game/02_Blueprints/ProceduralMap/BP_Room_Base.BP_Room_Base_C|GetConexionsArray _output_get) (Math|Random|RandomIntegerinRange 0 (- (Utilities|Array|Length (Variables|/Game/02_Blueprints/ProceduralMap/BP_Room_Base.BP_Room_Base_C|GetConexionsArray _output_get)) 1))))
    (Transformation|SetActorTransform (Variables|Default|GetCurrentRoom) (Math|Transform|ComposeTransforms (Math|Transform|ComposeTransforms (Math|Transform|InvertTransform (Transformation|GetRelativeTransform (Variables|Default|GetCurrentNewRoomDoor))) (Math|Transform|MakeTransform "0, 0, 0" (Math|Rotator|MakeRotator 0.0 0.0 1.8e+02))) (Transformation|GetWorldTransform (Variables|Default|GetCurentlyTestedFreeConnexion))))
    (bind _doesoverlap (CallFunction|CheckOverlap))
    (return _doesoverlap)
    (else
      (return true))))

(fn CloseDoor
  (params (Door :type Scene%20Component%20Object%20Reference))
  (Game|SpawnActorfromClass "/Game/02_Blueprints/ProceduralMap/ClosedDoor.ClosedDoor_C" (Math|Conversions|ToTransform(Vector) (Transformation|GetWorldLocation Door)) "Undefined" "MultiplyWithRoot" 0 0))

(fn FindARandomWeighted
  (LocalVariables|SetFound false)
  (Utilities|FlowControl|Sequence
    (:then_0
      ;[0.15 0.1342 0.006468 0.5] Calculate overall weight if the room class can be used
      (Variables|Default|SetTotalWeightValue 0)
      (for _array_element (Variables|Default|GetFloorValidModules)
        (Variables|Default|SetTotalWeightValue (+ (.Weight (Utilities|Struct|BreakS_RoomStruct _array_element)) (Variables|Default|GetTotalWeightValue)))))
    (:then_1
      ;[0.07872 0.02388 0.15 0.5] Randomly finds the room class to use, based on weights
      (if (> (Variables|Default|GetTotalWeightValue) 0)
        (LocalVariables|SetRandomWeightValue (Math|Random|RandomIntegerinRange 0 (- (Variables|Default|GetTotalWeightValue) 1)))
        (LocalVariables|SetRunningWeightValue 0)
        (bind _array_element_2 (Utilities|Array|ForEachLoopwithBreak (Variables|Default|GetFloorValidModules) :!label _label)
          (:LoopBody
            (LocalVariables|SetRunningWeightValue (+ (.Weight (Utilities|Struct|BreakS_RoomStruct _array_element_2)) (LocalVariables|GetRunningWeightValue)))
            (bind _output_get (LocalVariables|SetFound (< (LocalVariables|GetRandomWeightValue) (LocalVariables|GetRunningWeightValue))))
            (if _output_get
              (Variables|Default|SetCurrentlyTestedRoom _array_element_2)
              (goto _label Break)))
          (:Completed
            (return (LocalVariables|GetFound))))
        (else
          (return false))))))

(fn SaveRoomData
  (bind _currentroom (Variables|Default|GetCurrentRoom))
  (Utilities|Array|AddUnique (Variables|Default|GetSavedRoomData) (Utilities|Struct|MakeS_RoomData (Utilities|GetClass _currentroom) (Variables|/Game/02_Blueprints/ProceduralMap/BP_Room_Base.BP_Room_Base_C|GetRoomType _currentroom) (Transformation|GetActorTransform _currentroom) (Variables|/Game/02_Blueprints/ProceduralMap/BP_Room_Base.BP_Room_Base_C|GetMinimapVersion _currentroom))))

(fn ModifyCurrentRoom/Floor
  (bind _currentlytestedroom (Variables|Default|GetCurrentlyTestedRoom))
  (bind _floorvalidmodules (Variables|Default|GetFloorValidModules))
  (bind _returnvalue (Utilities|Array|FindItem _floorvalidmodules _currentlytestedroom))
  (bind _output (Utilities|Array|Get(acopy) _floorvalidmodules _returnvalue))
  (bind _floorcurrentroomamount (Utilities|Struct|BreakS_RoomStruct _output))
  ;[0.04158 0.06193 0.15 0.5] Increment the room type spawned, if not available anymore, removed from floor avaiability array
  (LocalVariables|SetIndex _returnvalue)
  (Utilities|Map|Add _floorcurrentroomamount (Variables|Default|GetCurrentFloor) (+ (.Value (Utilities|Map|Find _floorcurrentroomamount (Variables|Default|GetCurrentFloor))) 1))
  (if (.ReturnValue (Utilities|Map|Find (.FloorMaxRoom (Utilities|Struct|BreakS_RoomStruct (Utilities|Array|Get(acopy) (Variables|Default|GetFloorValidModules) (LocalVariables|GetIndex)))) (Variables|Default|GetCurrentFloor)))
    (if (not (> (.Value (Utilities|Map|Find (.FloorMaxRoom (Utilities|Struct|BreakS_RoomStruct (Utilities|Array|Get(acopy) (Variables|Default|GetFloorValidModules) (LocalVariables|GetIndex)))) (Variables|Default|GetCurrentFloor))) (.Value (Utilities|Map|Find (.FloorCurrentRoomAmount (Utilities|Struct|BreakS_RoomStruct (Utilities|Array|Get(acopy) (Variables|Default|GetFloorValidModules) (LocalVariables|GetIndex)))) (Variables|Default|GetCurrentFloor)))))
      (Utilities|Array|RemoveIndex (Variables|Default|GetFloorValidModules) (LocalVariables|GetIndex)))))

(fn CheckRoomAvaibility(maxAmount)
  (params (Room%20struct :type S%20Room%20Struct%20Structure))
  (bind (_roomclass _weight _floormaxroom _floorcurrentroomamount) (Utilities|Struct|BreakS_RoomStruct Room%20struct))
  (bind _currentfloor (Variables|Default|GetCurrentFloor))
  (bind (_value _returnvalue) (Utilities|Map|Find _floormaxroom _currentfloor))
  (if _returnvalue
    (if (> _value (.Value (Utilities|Map|Find _floorcurrentroomamount (Variables|Default|GetCurrentFloor))))
      (Development|PrintString "Hello")
      (return true)
      (else
        (return false)))
    (else
      (return true))))