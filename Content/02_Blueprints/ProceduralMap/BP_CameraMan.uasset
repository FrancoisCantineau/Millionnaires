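; BP_CameraMan drives a SceneCaptureComponent2D over the procedural map, updating which rooms it hides as elevators change floors.
; Ten seconds after BeginPlay, it sets the capture's HiddenActors to the Map's ReturnRoomsForFloor result for floor 0.
; It then binds to every BP_Elevator's new-floor-reached event, replacing the hidden list with that query's result for the reached floor.
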(event Custom|CustomEvent
  (params (NewFloor :type Integer))
  (bind _rooms (Default|ReturnRoomsforFloor (Variables|Default|GetMap) NewFloor))
  (Variables|/Script/Engine.SceneCaptureComponent|SetHiddenActors (Variables|Default|GetSceneCaptureComponent2D) _rooms))

(event EventBeginPlay
  (Utilities|FlowControl|Delay 1e+01)
  (bind _rooms (Default|ReturnRoomsforFloor (Variables|Default|GetMap)))
  (Variables|/Script/Engine.SceneCaptureComponent|SetHiddenActors (Variables|Default|GetSceneCaptureComponent2D) _rooms)
  (bind _outactors (Actor|GetAllActorsOfClass "/Game/02_Blueprints/ProceduralMap/BP_Elevator.BP_Elevator_C"))
  (for _array_element _outactors
    (EventDispatchers|BindEventtoNewFloorReached _array_element (delegate Custom|CustomEvent))))

(event Collision|EventActorBeginOverlap
  (params (OtherActor :type Actor%20Object%20Reference)))

(event EventTick
  (params (DeltaSeconds :type Float%20%28single-precision%29)))

(fn ConstructionScript)