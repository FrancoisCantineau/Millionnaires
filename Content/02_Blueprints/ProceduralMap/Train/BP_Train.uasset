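; BP_Train is a train actor whose Cube rides along the Rai spline once the player pawn overlaps its Box.
; The overlap enables Tick, which advances a stored distance and sets the Cube's relative location and rotation from the spline.
; Speed scales with the remaining distance to spline point 1, capped at SplineSPeed, so the train eases into that point.
; Tick also debug-prints the target distance, and leftover Timeline movement logic never runs.
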(event OnComponentBeginOverlap(Box)
  (params (OverlappedComponent :type Primitive%20Component%20Object%20Reference) (OtherActor :type Actor%20Object%20Reference) (OtherComp :type Primitive%20Component%20Object%20Reference) (OtherBodyIndex :type Integer) (bFromSweep :type Boolean) (SweepResult :type Hit%20Result%20Structure%20%28by%20ref%29))
  (if (== OtherActor (Game|Player|GetPlayerPawn 0))
    (CallFunction|StartTrain)))

(event Custom|StartTrain
  (Actor|Tick|SetActorTickEnabled true))

(event EventBeginPlay)

(event Collision|EventActorBeginOverlap
  (params (OtherActor :type Actor%20Object%20Reference)))

(event EventTick
  (params (DeltaSeconds :type Float%20%28single-precision%29))
  (bind _splinespeed (Variables|Default|GetSplineSPeed))
  (bind _rai (Variables|Default|Getrai))
  (bind _returnvalue (Spline|GetDistanceAlongSplineatSplinePoint _rai 1))
  (Development|PrintString (Utilities|String|ToString(Float) _returnvalue))
  (bind _output_get (Variables|Default|SetDistanceAlongTheSpline (+ (* (Math|Float|Clamp(Float) (* (Math|Float|MakeLiteralFloat (/ (- _returnvalue (Variables|Default|GetDistanceAlongTheSpline)) 1e+02)) _splinespeed) 0.0 _splinespeed) DeltaSeconds) (Variables|Default|GetDistanceAlongTheSpline))))
  (Transformation|SetRelativeTransform (Variables|Default|GetCube) (Math|Transform|MakeTransform (.location (Spline|GetTransformatDistanceAlongSpline (Variables|Default|Getrai) _output_get "Local" false)) (.rotation (Spline|GetTransformatDistanceAlongSpline (Variables|Default|Getrai) _output_get "Local" false)) "1.000000,1.000000,1.000000") false false))

(fn ConstructionScript)