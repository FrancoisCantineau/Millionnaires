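; Procedural map generator that builds floors of connected rooms, each new floor starting from an elevator spawned below the previous one.
; It snaps weighted-random room types onto random free doors, with optional transition pieces and per-floor type caps.
; Overlapping rooms are destroyed and other types tried; exhausted doors are sealed, and running out restarts the floor.
; Saved room data feeds a 3D map; shortcut creation is unwired.
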(event Custom|SpawnNextRoom
  ;[0.15 0.1165 0.04275 0.5] Spawns a room
  (Variables|Default|GetCurentlyTestedFreeConnexion
    (:then
      (bind _spawnblocked_ (CallFunction|SpawnRoom&Test :!label _label))
      (if _spawnblocked_
        (bind _returnvalue (Utilities|Array|RemoveItem (Variables|Default|GetCurrentTestedRoomsType) (Variables|Default|GetCurrentlyTestedRoomType)))
        (if _returnvalue
          (if (Utilities|Array|IsEmpty (Variables|Default|GetCurrentTestedRoomsType))
            (Utilities|Array|RemoveItem (Variables|Doors/Connexions|GetFreeDoorsList) (Variables|Default|GetCurentlyTestedFreeConnexion) :!label _label_2)
            (Utilities|Array|Clear (Variables|Default|GetCurrentTestedRoomsType))
            (for _array_element (Variables|Default|GetValidRoomTypeForThisFloor)
              (Utilities|Array|AddUnique (Variables|Default|GetCurrentTestedRoomsType) _array_element))
            (CallFunction|CloseDoor (Variables|Default|GetCurentlyTestedFreeConnexion))
            (Variables|Default|SetCurentlyTestedFreeConnexion 0)
            (CallFunction|SpawnNextRoom)
            (else
              (Variables|Default|SetCurrentlyTestedRoomType "")
              (CallFunction|SpawnNextRoom)))
          (else
            (goto _label_2)))
        (else
          (CallFunction|SaveRoomData)
          (CallFunction|ModifyCurrentRoom/Floor)
          (Utilities|Array|Clear (Variables|Default|GetCurrentTestedRoomsType))
          (for _array_element_2 (Variables|Default|GetValidRoomTypeForThisFloor)
            (Utilities|Array|AddUnique (Variables|Default|GetCurrentTestedRoomsType) _array_element_2))
          (for _array_element_3 (Variables|/Game/02_Blueprints/ProceduralMap/BP_Room_Base.BP_Room_Base_C|GetDoorsArray (Variables|Default|GetCurrentRoomRef))
            (bind _structout (Utilities|Struct|SetmembersinS_DoorData (Variables|/Game/02_Blueprints/ProceduralMap/DoorArrow.DoorArrow_C|GetDoorData _array_element_3) (Variables|Default|GetCurrentRoomRef)))
            (Variables|/Game/02_Blueprints/ProceduralMap/DoorArrow.DoorArrow_C|SetDoorData _array_element_3 _structout))
          (Utilities|Array|AppendArray (Variables|Doors/Connexions|GetFreeDoorsList) (Variables|/Game/02_Blueprints/ProceduralMap/BP_Room_Base.BP_Room_Base_C|GetDoorsArray (Variables|Default|GetCurrentRoomRef)))
          (Utilities|Array|AppendArray (Variables|Doors/Connexions|GetFreeConnexionsList) (Variables|/Game/02_Blueprints/ProceduralMap/BP_Room_Base.BP_Room_Base_C|GetConexionsArray (Variables|Default|GetCurrentRoomRef)))
          (Utilities|Array|RemoveItem (Variables|Doors/Connexions|GetFreeDoorsList) (Variables|Default|GetCurentlyTestedFreeConnexion))
          (Utilities|Array|RemoveItem (Variables|Doors/Connexions|GetFreeDoorsList) (Variables|Doors/Connexions|GetCurrentNewRoomDoor))
          (Utilities|Array|AddUnique (Variables|Default|GetSpawnedRooms%20for%20this%20floor) (Variables|Default|GetCurrentRoomRef))
          (Variables|Default|SetCurentlyTestedFreeConnexion 0)
          (Math|Integer|IncrementInt (Variables|Default|GetCurrentRoomSpawnIndex)
            (:%20%20
              (if (> (Variables|Default|GetMaxRooms) (Variables|Default|GetCurrentRoomSpawnIndex))
                (Utilities|FlowControl|Delay 0.0)
                (CallFunction|SpawnNextRoom)
                (else
                  (Development|PrintString "GINIT")
                  (CallFunction|CreateShortcut)
                  (Default|Build3DMap (Variables|Default|Get3dMap) (Variables|Default|GetSavedRoomData))
                  (CallFunction|SetupNextFloor))))))))
    (:else
      (bind _output_get (Variables|Default|SetCurentlyTestedFreeConnexion (.OutItem (Utilities|Array|Random (Variables|Doors/Connexions|GetFreeDoorsList)))))
      (Utilities|IsValid _output_get
        (:Is%20Valid
          (goto _label))
        (:Is%20Not%20Valid
          (CallFunction|RestartGeneration))))))

(event Custom|CreateShortcut)

(event Custom|RestartGeneration
  ;[0.03747 0.15 0.04797 0.5] Restarts the current floor generation (not the whole generation tho)
  (for _array_element (Variables|Default|Getclosed%20doors)
    (Actor|DestroyActor _array_element))
  (for _array_element_2 (Variables|Default|GetSpawnedRooms%20for%20this%20floor)
    (if (not (== _array_element_2 (Variables|Default|GetFirstRoomForThisFloorRef)))
      (Actor|DestroyActor _array_element_2)))
  (Utilities|Array|Clear (Variables|Default|GetSavedRoomData))
  (for _array_element_3 (Variables|Default|GetUsableRoomType)
    (Utilities|Map|Clear (.FloorCurrentRoomAmount (Utilities|Struct|BreakS_RoomStruct _array_element_3))))
  (Utilities|FlowControl|Delay 0.0)
  (CallFunction|StartGeneration))

(event Custom|StartGeneration
  ;[0.15 0.01276 0.01276 0.5] Setup the starting of a floor generation and launch next steps
  (CallFunction|SetupArray/Variables)
  (CallFunction|SpawnNextRoom))

(event Custom|SetupNextFloor
  ;[0.15 0.1467 0.004874 0.5] Setup next floor initialization. Creates a new base room for the current floor
  (Utilities|Array|Clear (Variables|Default|Getclosed%20doors))
  (Math|Integer|IncrementInt (Variables|Default|GetCurrentFloor)
    (:%20%20
      (if (< (Variables|Default|GetCurrentFloor) 4)
        (bind _array_element (Utilities|Array|ForEachLoopwithBreak (Variables|Default|GetSavedRoomData) :!label _label)
          (:LoopBody
            (if (== (.Floor (Utilities|Struct|BreakS_RoomData _array_element)) (- (Variables|Default|GetCurrentFloor) 1))
              (if (Utilities|Enum|Equal(Enum) (Variables|/Game/02_Blueprints/ProceduralMap/BP_Room_Base.BP_Room_Base_C|GetRoomType (.RoomRef (Utilities|Struct|BreakS_RoomData _array_element))) "NewEnumerator3")
                (bind _returnvalue (Game|SpawnActorfromClass "/Game/02_Blueprints/ProceduralMap/BP_Elevator.BP_Elevator_C" (Math|Transform|MakeTransform (Math|Vector|MakeVector (.x (.location (Transformation|GetActorTransform (.RoomRef (Utilities|Struct|BreakS_RoomData _array_element))))) (.y (.location (Transformation|GetActorTransform (.RoomRef (Utilities|Struct|BreakS_RoomData _array_element))))) (- (.z (.location (Transformation|GetActorTransform (.RoomRef (Utilities|Struct|BreakS_RoomData _array_element))))) 3e+03)) (.rotation (Transformation|GetActorTransform (.RoomRef (Utilities|Struct|BreakS_RoomData _array_element)))) (.scale (Transformation|GetActorTransform (.RoomRef (Utilities|Struct|BreakS_RoomData _array_element))))) "AlwaysSpawn" "MultiplyWithRoot" 0 0))
                (bind _asbp_elevator (Utilities|Casting|CastToBP_Elevator (.RoomRef (Utilities|Struct|BreakS_RoomData _array_element))))
                (Default|AddNewFloor _asbp_elevator _returnvalue (Variables|Default|GetCurrentFloor))
                (Variables|Default|SetFirstRoomForThisFloorRef _returnvalue)
                (goto _label Break))))
          (:Completed
            (CallFunction|StartGeneration)))))))

(event Custom|SetupArray/Variables
  (bind _spawnedrooms_for_this_floor (Variables|Default|GetSpawnedRooms%20for%20this%20floor))
  (Variables|Default|SetCurrentRoomRef (Variables|Default|GetFirstRoomForThisFloorRef))
  (CallFunction|SaveRoomData)
  (Utilities|Array|Clear (Variables|Doors/Connexions|GetFreeConnexionsList))
  (Utilities|Array|Clear (Variables|Doors/Connexions|GetFreeDoorsList))
  ;[0.0129 0.15 0.1342 0.5] Setup cariables/array for the generation
  (for _array_element (Variables|/Game/02_Blueprints/ProceduralMap/BP_Room_Base.BP_Room_Base_C|GetDoorsArray (Variables|Default|GetFirstRoomForThisFloorRef))
    (bind _structout (Utilities|Struct|SetmembersinS_DoorData (Variables|/Game/02_Blueprints/ProceduralMap/DoorArrow.DoorArrow_C|GetDoorData _array_element) (Variables|Default|GetCurrentRoomRef)))
    (Variables|/Game/02_Blueprints/ProceduralMap/DoorArrow.DoorArrow_C|SetDoorData _array_element _structout))
  (Utilities|Array|AppendArray (Variables|Doors/Connexions|GetFreeDoorsList) (Variables|/Game/02_Blueprints/ProceduralMap/BP_Room_Base.BP_Room_Base_C|GetDoorsArray (Variables|Default|GetFirstRoomForThisFloorRef)))
  (Utilities|Array|AppendArray (Variables|Doors/Connexions|GetFreeConnexionsList) (Variables|/Game/02_Blueprints/ProceduralMap/BP_Room_Base.BP_Room_Base_C|GetConexionsArray (Variables|Default|GetFirstRoomForThisFloorRef)))
  (Utilities|Array|Clear _spawnedrooms_for_this_floor)
  (Utilities|Array|AddUnique _spawnedrooms_for_this_floor (Variables|Default|GetFirstRoomForThisFloorRef))
  (Variables|Default|SetCurrentRoomSpawnIndex 0)
  (Variables|Doors/Connexions|SetCurrentNewRoomDoor 0)
  (Variables|Default|SetCurentlyTestedFreeConnexion 0)
  (Variables|Default|SetCurrentRoomRef 0)
  (Utilities|Array|Clear (Variables|Default|GetValidRoomTypeForThisFloor))
  (Utilities|Array|AppendArray (Variables|Default|GetValidRoomTypeForThisFloor) (Variables|Default|GetUsableRoomType))
  (Utilities|Array|Clear (Variables|Default|GetCurrentTestedRoomsType))
  (for _array_element_2 (Variables|Default|GetValidRoomTypeForThisFloor)
    (if (.ReturnValue (Utilities|Map|Find (.FloorMaxRoom (Utilities|Struct|BreakS_RoomStruct _array_element_2)) (Variables|Default|GetCurrentFloor)))
      (if (== (.Value (Utilities|Map|Find (.FloorMaxRoom (Utilities|Struct|BreakS_RoomStruct _array_element_2)) (Variables|Default|GetCurrentFloor))) 0)
        (Utilities|Array|RemoveItem (Variables|Default|GetValidRoomTypeForThisFloor) _array_element_2)
        (else
          (Utilities|Array|AddUnique (Variables|Default|GetCurrentTestedRoomsType) _array_element_2 :!label _label)))
      (else
        (goto _label)))))

(event EventBeginPlay
  (bind _returnvalue (Game|SpawnActorfromClass (Variables|Default|GetFirstRoom) (Math|Transform|MakeTransform "0, 0, 0" "0, 0, 0" "1.000000,1.000000,1.000000") "Undefined" "MultiplyWithRoot" 0 0))
  (Variables|Default|SetFirstRoomForThisFloorRef _returnvalue)
  (CallFunction|StartGeneration))

(fn ConstructionScript)

(fn CheckOverlap
  (bind _overlappingarray (Variables|Default|GetOverlappingArray))
  (for _array_element (Components|GetChildrenComponents (Variables|/Game/02_Blueprints/ProceduralMap/BP_Room_Base.BP_Room_Base_C|GetOverlappingComp (Variables|Default|GetCurrentRoomRef)) false)
    (bind _asbox_collision (Utilities|Casting|CastToBoxComponent _array_element))
    (Utilities|Array|AppendArray (Variables|Default|GetOverlappingArray) (Class|PrimitiveComponent|GetOverlappingComponents _asbox_collision)))
  (if (Utilities|Array|IsEmpty _overlappingarray)
    (return false)
    (else
      (Utilities|Array|Clear _overlappingarray)
      (Actor|DestroyActor (Variables|Default|GetCurrentRoomRef))
      (Variables|Default|SetCurrentRoomRef 0)
      (return true))))

(fn SpawnRoom&Test
  ;[0.15 0.09913 0 0.5] SpawnNextRoom
  (bind _randomfound (CallFunction|FindARandomWeighted))
  (if _randomfound
    (bind _returnvalue (Game|SpawnActorfromClass (.RoomClass (Utilities|Struct|BreakS_RoomStruct (Variables|Default|GetCurrentlyTestedRoomType))) (Transformation|GetWorldTransform (Variables|/Game/02_Blueprints/ProceduralMap/DoorArrow.DoorArrow_C|GetArrow (Variables|Default|GetCurentlyTestedFreeConnexion))) "AlwaysSpawn" "MultiplyWithRoot" 0 0))
    (bind _output_get (Variables|Default|SetCurrentRoomRef _returnvalue))
    (bind _output_get_2 (Variables|Doors/Connexions|SetCurrentNewRoomDoor (Utilities|Array|Get(acopy) (Variables|/Game/02_Blueprints/ProceduralMap/BP_Room_Base.BP_Room_Base_C|GetDoorsArray _output_get) (Math|Random|RandomIntegerinRange 0 (- (Utilities|Array|Length (Variables|/Game/02_Blueprints/ProceduralMap/BP_Room_Base.BP_Room_Base_C|GetDoorsArray _output_get)) 1)))))
    (Utilities|IsValid _output_get_2
      (:Is%20Valid
        (bind (_transform _foundtransition) (CallFunction|DoorTransition))
        (if _foundtransition
          (bind _newparam1 (CallFunction|CalculateRoomPosition _transform))
          (LocalVariables|SetNewLocalVar _newparam1)
          (else
            (bind _newparam1_2 (CallFunction|CalculateRoomPosition (Transformation|GetWorldTransform (Variables|/Game/02_Blueprints/ProceduralMap/DoorArrow.DoorArrow_C|GetArrow (Variables|Default|GetCurentlyTestedFreeConnexion)))))
            (LocalVariables|SetNewLocalVar _newparam1_2)))
        (Transformation|SetActorTransform (Variables|Default|GetCurrentRoomRef) (LocalVariables|GetNewLocalVar))
        (bind _doesoverlap (CallFunction|CheckOverlap))
        (return _doesoverlap)))
    (else
      (return true))))

(fn CloseDoor
  (params (Door :type Door%20Arrow%20Object%20Reference))
  (bind _returnvalue (Game|SpawnActorfromClass "/Game/02_Blueprints/ProceduralMap/ClosedDoor.ClosedDoor_C" (Math|Conversions|ToTransform(Vector) (Transformation|GetWorldLocation (Variables|/Game/02_Blueprints/ProceduralMap/DoorArrow.DoorArrow_C|GetArrow Door))) "Undefined" "MultiplyWithRoot" 0 0))
  (Utilities|Array|AddUnique (Variables|Default|Getclosed%20doors) _returnvalue))

(fn FindARandomWeighted
  (LocalVariables|SetFound false)
  (Utilities|FlowControl|Sequence
    (:then_0
      ;[0.15 0.1342 0.006468 0.5] Calculate overall weight if the room class can be used
      (Variables|Default|SetTotalWeightValue 0)
      (for _array_element (Variables|Default|GetCurrentTestedRoomsType)
        (if (not (Utilities|Enum|Equal(Enum) (Variables|/Game/02_Blueprints/ProceduralMap/BP_Room_Base.BP_Room_Base_C|GetRoomType (.RoomRef (Utilities|Struct|BreakS_DoorData (Variables|/Game/02_Blueprints/ProceduralMap/DoorArrow.DoorArrow_C|GetDoorData (Variables|Default|GetCurentlyTestedFreeConnexion))))) "NewEnumerator0"))
          _
          (else
            (Utilities|Casting|CastToBP_Hallway_BaseClass (.RoomClass (Utilities|Struct|BreakS_RoomStruct _array_element)))))
        (Variables|Default|SetTotalWeightValue (+ (.Weight (Utilities|Struct|BreakS_RoomStruct _array_element)) (Variables|Default|GetTotalWeightValue)))))
    (:then_1
      ;[0.07872 0.02388 0.15 0.5] Randomly finds the room class to use, based on weights
      (if (> (Variables|Default|GetTotalWeightValue) 0)
        (LocalVariables|SetRandomWeightValue (Math|Random|RandomIntegerinRange 0 (- (Variables|Default|GetTotalWeightValue) 1)))
        (LocalVariables|SetRunningWeightValue 0)
        (bind _array_element_2 (Utilities|Array|ForEachLoopwithBreak (Variables|Default|GetCurrentTestedRoomsType) :!label _label)
          (:LoopBody
            (if (not (Utilities|Enum|Equal(Enum) (Variables|/Game/02_Blueprints/ProceduralMap/BP_Room_Base.BP_Room_Base_C|GetRoomType (.RoomRef (Utilities|Struct|BreakS_DoorData (Variables|/Game/02_Blueprints/ProceduralMap/DoorArrow.DoorArrow_C|GetDoorData (Variables|Default|GetCurentlyTestedFreeConnexion))))) "NewEnumerator0"))
              _
              (else
                (Utilities|Casting|CastToBP_Hallway_BaseClass (.RoomClass (Utilities|Struct|BreakS_RoomStruct _array_element_2)))))
            (LocalVariables|SetRunningWeightValue (+ (.Weight (Utilities|Struct|BreakS_RoomStruct _array_element_2)) (LocalVariables|GetRunningWeightValue)))
            (bind _output_get (LocalVariables|SetFound (< (LocalVariables|GetRandomWeightValue) (LocalVariables|GetRunningWeightValue))))
            (if _output_get
              (Variables|Default|SetCurrentlyTestedRoomType _array_element_2)
              (goto _label Break)))
          (:Completed
            (return (LocalVariables|GetFound))))
        (else
          (return false))))))

(fn SaveRoomData
  (bind _currentroomref (Variables|Default|GetCurrentRoomRef))
  (Utilities|Array|AddUnique (Variables|Default|GetSavedRoomData) (Utilities|Struct|MakeS_RoomData (Utilities|GetClass _currentroomref) (Variables|/Game/02_Blueprints/ProceduralMap/BP_Room_Base.BP_Room_Base_C|GetRoomType _currentroomref) (Transformation|GetActorTransform _currentroomref) (Variables|/Game/02_Blueprints/ProceduralMap/BP_Room_Base.BP_Room_Base_C|GetMinimapVersion _currentroomref) (Variables|Default|GetCurrentFloor) _currentroomref)))

(fn ModifyCurrentRoom/Floor
  (bind _currentlytestedroomtype (Variables|Default|GetCurrentlyTestedRoomType))
  (bind _validroomtypeforthisfloor (Variables|Default|GetValidRoomTypeForThisFloor))
  (bind _returnvalue (Utilities|Array|FindItem _validroomtypeforthisfloor _currentlytestedroomtype))
  (bind _output (Utilities|Array|Get(acopy) _validroomtypeforthisfloor _returnvalue))
  (bind _floorcurrentroomamount (Utilities|Struct|BreakS_RoomStruct _output))
  ;[0.04158 0.06193 0.15 0.5] Increment the room type spawned, if not available anymore, removed from floor avaiability array
  (LocalVariables|SetIndex _returnvalue)
  (Utilities|Map|Add _floorcurrentroomamount (Variables|Default|GetCurrentFloor) (+ (.Value (Utilities|Map|Find _floorcurrentroomamount (Variables|Default|GetCurrentFloor))) 1))
  (if (.ReturnValue (Utilities|Map|Find (.FloorMaxRoom (Utilities|Struct|BreakS_RoomStruct (Utilities|Array|Get(acopy) (Variables|Default|GetValidRoomTypeForThisFloor) (LocalVariables|GetIndex)))) (Variables|Default|GetCurrentFloor)))
    (if (not (> (.Value (Utilities|Map|Find (.FloorMaxRoom (Utilities|Struct|BreakS_RoomStruct (Utilities|Array|Get(acopy) (Variables|Default|GetValidRoomTypeForThisFloor) (LocalVariables|GetIndex)))) (Variables|Default|GetCurrentFloor))) (.Value (Utilities|Map|Find (.FloorCurrentRoomAmount (Utilities|Struct|BreakS_RoomStruct (Utilities|Array|Get(acopy) (Variables|Default|GetValidRoomTypeForThisFloor) (LocalVariables|GetIndex)))) (Variables|Default|GetCurrentFloor)))))
      (Utilities|Array|RemoveIndex (Variables|Default|GetValidRoomTypeForThisFloor) (LocalVariables|GetIndex)))))

(fn CheckRoomAvaibility(maxAmount)
  (params (Room%20struct :type S%20Room%20Struct%20Structure))
  (bind (_roomclass _weight _floormaxroom _floorcurrentroomamount) (Utilities|Struct|BreakS_RoomStruct Room%20struct))
  (bind _currentfloor (Variables|Default|GetCurrentFloor))
  (bind (_value _returnvalue) (Utilities|Map|Find _floormaxroom _currentfloor))
  (if _returnvalue
    (if (> _value (.Value (Utilities|Map|Find _floorcurrentroomamount (Variables|Default|GetCurrentFloor))))
      (return true)
      (else
        (return false)))
    (else
      (return true))))

(fn ReturnRoomsforFloor
  (params (Floor :type Integer))
  (for _array_element (Variables|Default|GetSavedRoomData)
    (if (!= (.Floor (Utilities|Struct|BreakS_RoomData _array_element)) Floor)
      (Development|PrintString "Hello")
      (Utilities|Array|AddUnique (LocalVariables|GetRoomsArray) (.RoomRef (Utilities|Struct|BreakS_RoomData _array_element)))))
  (return (LocalVariables|GetRoomsArray)))

(fn DoorTransition
  (bind _currentnewroomdoor (Variables|Doors/Connexions|GetCurrentNewRoomDoor))
  (bind _roomtransition (Variables|Default|GetRoomTransition))
  (bind _curentlytestedfreeconnexion (Variables|Default|GetCurentlyTestedFreeConnexion))
  (bind _doordata (Variables|/Game/02_Blueprints/ProceduralMap/DoorArrow.DoorArrow_C|GetDoorData _currentnewroomdoor))
  (bind _doordata_2 (Variables|/Game/02_Blueprints/ProceduralMap/DoorArrow.DoorArrow_C|GetDoorData _curentlytestedfreeconnexion))
  (bind _doortype (Utilities|Struct|BreakS_DoorData _doordata))
  (bind _doortype_2 (Utilities|Struct|BreakS_DoorData _doordata_2))
  (bind _s_doorpairkey (Utilities|Struct|MakeS_DoorPairKey _doortype _doortype_2))
  (bind (_value _returnvalue) (Utilities|Map|Find _roomtransition _s_doorpairkey))
  (if _returnvalue
    (bind _returnvalue_2 (Game|SpawnActorfromClass _value (Transformation|GetActorTransform (Variables|Default|GetCurentlyTestedFreeConnexion)) "AlwaysSpawn" "MultiplyWithRoot" 0 0))
    (return (Transformation|GetWorldTransform (Variables|/Game/02_Blueprints/ProceduralMap/BP_DoorTransitionBase.BP_DoorTransitionBase_C|GetBROOMPOSItion _returnvalue_2)) _returnvalue)))

(fn CalculateRoomPosition
  (params (ArrowTransofrm :type Transform))
  ;[0.15 0.15 0.15 0.5] returns the position of the room,  oriented and placed using a relative component
  (return (Math|Transform|ComposeTransforms (Math|Transform|ComposeTransforms (Math|Transform|InvertTransform (Math|Transform|MakeRelativeTransform (Transformation|GetActorTransform (Variables|Doors/Connexions|GetCurrentNewRoomDoor)) (Transformation|GetActorTransform (Variables|Default|GetCurrentRoomRef)))) (Math|Transform|MakeTransform "0, 0, 0" (Math|Rotator|MakeRotator 0.0 0.0 1.8e+02))) ArrowTransofrm)))