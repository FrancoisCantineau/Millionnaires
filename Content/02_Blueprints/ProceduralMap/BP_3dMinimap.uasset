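; BP_3dMinimap builds a miniature 3D version of the procedural map from arrays of room data, organised by floor.
; Each Build3DMap call adds a scene component for a floor, attaches spawned MiniVersion room actors to it, then scales down the child component at the incremented floor index.
; The new floor is hidden and floor 0 shown; ShowFloor only unhides the indexed floor and its children, without hiding others.
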(event Custom|Build3DMap
  (params (ArrayRoomData :type Array%20of%20S%20Room%20Data%20Structures))
  ;[0.15 0.6812 0.15 0.5] Build a mini version 3d based of an array of given rooms. Each new call will create a new scene comp, parenting entirely the floor
  (bind _returnvalue (AddComponent|AddSceneComponent false))
  (bind _output_get (Variables|Default|SetCurrentFloorComp _returnvalue))
  (Transformation|AttachComponentToComponent _output_get (Variables|Default|GetDefaultSceneRoot) "None" "KeepRelative" "KeepRelative" "KeepRelative" true)
  (Math|Integer|IncrementInt (Variables|Default|GetCurrentFloor)
    (:%20%20
      (for _array_element ArrayRoomData
        (if (Utilities|IsValidClass (.MiniVersion (Utilities|Struct|BreakS_RoomData _array_element)))
          (bind _returnvalue_2 (Game|SpawnActorfromClass (.MiniVersion (Utilities|Struct|BreakS_RoomData _array_element)) (.Position (Utilities|Struct|BreakS_RoomData _array_element)) "AlwaysSpawn" "MultiplyWithRoot" 0 0))
          (Transformation|AttachComponentToComponent _returnvalue_2 (Variables|Default|GetCurrentFloorComp) "None" "KeepWorld" "KeepWorld" "KeepWorld" true)))
      (Transformation|SetWorldScale3D (Components|GetChildComponent (Variables|Default|GetDefaultSceneRoot) (Variables|Default|GetCurrentFloor)) "0.030000,0.030000,0.030000")
      (Development|SetHiddeninGame (Variables|Default|GetCurrentFloorComp) true true)
      (CallFunction|ShowFloor)
      (Variables|Default|SetCurrentFloorComp 0))))

(event Custom|ShowFloor
  (params (Floor :type Integer))
  ;[0.15 0.01641 0.01641 0.5] Set the visibility for a given floor
  (Development|SetHiddeninGame (Components|GetChildComponent (Variables|Default|GetDefaultSceneRoot) Floor) false true))

(fn ConstructionScript)