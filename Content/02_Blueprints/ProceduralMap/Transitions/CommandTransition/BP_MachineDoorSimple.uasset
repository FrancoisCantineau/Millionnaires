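; BP_MachineDoorSimple is a simple automatic sliding door for the procedural map's command transition.
; When the player pawn enters the Collision volume, a timeline lerps the SMDoorL mesh from its starting relative location to 300 units higher on Z.
; When the pawn leaves, the same timeline reverses to lower the door.
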(event OnComponentBeginOverlap(Collision)
  (params (OverlappedComponent :type Primitive%20Component%20Object%20Reference) (OtherActor :type Actor%20Object%20Reference) (OtherComp :type Primitive%20Component%20Object%20Reference) (OtherBodyIndex :type Integer) (bFromSweep :type Boolean) (SweepResult :type Hit%20Result%20Structure%20%28by%20ref%29))
  (if (== OtherActor (Game|Player|GetPlayerPawn 0))
    (bind _newtrack_0 (Timeline|Timeline Play)
      (:Update
        (Transformation|SetRelativeLocation (Variables|Default|GetSM_Door_L) (Math|Vector|Lerp(Vector) (Variables|Default|GetOriginalPosition) (+ (Variables|Default|GetOriginalPosition) "0.000000,0.000000,300.000000") _newtrack_0) false false)))))

(event OnComponentEndOverlap(Collision)
  (params (OverlappedComponent :type Primitive%20Component%20Object%20Reference) (OtherActor :type Actor%20Object%20Reference) (OtherComp :type Primitive%20Component%20Object%20Reference) (OtherBodyIndex :type Integer))
  (if (== OtherActor (Game|Player|GetPlayerPawn 0))
    (bind _newtrack_0 (Timeline|Timeline Reverse)
      (:Update
        (Transformation|SetRelativeLocation (Variables|Default|GetSM_Door_L) (Math|Vector|Lerp(Vector) (Variables|Default|GetOriginalPosition) (+ (Variables|Default|GetOriginalPosition) "0.000000,0.000000,300.000000") _newtrack_0) false false)))))

(event EventBeginPlay
  (|CallParentFunction)
  (Variables|Default|SetOriginalPosition (Variables|/Script/Engine.SceneComponent|GetRelativeLocation (Variables|Default|GetSM_Door_L))))

(event Collision|EventActorBeginOverlap
  (params (OtherActor :type Actor%20Object%20Reference))
  (|CallParentFunction OtherActor) ; This node is disabled and will not be called.\nDrag off pins to build functionality.
)

(event EventTick
  (params (DeltaSeconds :type Float%20%28single-precision%29))
  (|CallParentFunction DeltaSeconds) ; This node is disabled and will not be called.\nDrag off pins to build functionality.
)

(fn ConstructionScript
  (|CallParentFunction))