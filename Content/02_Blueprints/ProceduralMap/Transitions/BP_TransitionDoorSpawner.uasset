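; Spawner for procedural map generation that builds, validates and removes transition door actors between rooms.
; It picks classes from TransitionMapping by door tag, spawning either a solo transition or a pair aligned on the first's attach arrow with the second rotated 180 degrees.
; Box overlap checks report collisions; otherwise the exit arrow's transform is returned.
; Validated transitions are recorded per attached room for targeted or full destruction.
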(event Custom|RemoveSpecificTransition
  (params (AttachedRoom :type BP%20Room%20Base%20Object%20Reference))
  (bind _array_element (Utilities|Array|ForEachLoopwithBreak (Variables|Default|GetTransitionsMappingWithRoom) :!label _label)
    (:LoopBody
      (if (== (.RoomAttached (Utilities|Struct|BreakS_TransitionsStruct _array_element)) AttachedRoom)
        (Utilities|IsValid (.TransitionA (Utilities|Struct|BreakS_TransitionsStruct _array_element))
          (:Is%20Valid
            (Actor|DestroyActor (.TransitionA (Utilities|Struct|BreakS_TransitionsStruct _array_element))))
          (:Is%20Not%20Valid
            _))
        (Utilities|IsValid (.TransitionB (Utilities|Struct|BreakS_TransitionsStruct _array_element))
          (:Is%20Valid
            (Actor|DestroyActor (.TransitionB (Utilities|Struct|BreakS_TransitionsStruct _array_element)))
            (Utilities|Array|RemoveItem (Variables|Default|GetTransitionsMappingWithRoom) _array_element)
            (goto _label Break)))))))

(event Custom|DestroyAllTransitions
  ;[0.8733 0.3824 0.2411 0.5] Destroys all transitions validated so far
  (for _array_element (Variables|Default|GetAllTransitions)
    (Utilities|IsValid _array_element
      (:Is%20Valid
        (Actor|DestroyActor _array_element))))
  (Variables|Default|SetCurrentTransitionA 0)
  (Variables|Default|SetCurrentTransitionB 0)
  (Utilities|Array|Clear (Variables|Default|GetAllTransitions)))

(event Custom|DestroyCurrentTransition
  ;[0.1788 0.9917 1 0.5] Clears current transitions
  (Variables|Default|GetCurrentTransitionA
    (:then
      (Actor|DestroyActor (Variables|Default|GetCurrentTransitionA))
      (Variables|Default|SetCurrentTransitionA 0))
    (:else
      _))
  (Variables|Default|GetCurrentTransitionB
    (:then
      (Actor|DestroyActor (Variables|Default|GetCurrentTransitionB))
      (Variables|Default|SetCurrentTransitionB 0))
    (:else)))

(event Custom|ValidateTransition
  (params (AttachedRoom :type BP%20Room%20Base%20Object%20Reference))
  ;[0.8589 0.8872 0.3156 0.5] Adds current transition to the overall array
  (Utilities|Array|AddUnique (Variables|Default|GetTransitionsMappingWithRoom) (Utilities|Struct|MakeS_TransitionsStruct AttachedRoom (Variables|Default|GetCurrentTransitionA) (Variables|Default|GetCurrentTransitionB)))
  (Utilities|Array|AddUnique (Variables|Default|GetAllTransitions) (Variables|Default|GetCurrentTransitionA))
  (Utilities|Array|AddUnique (Variables|Default|GetAllTransitions) (Variables|Default|GetCurrentTransitionB))
  (Variables|Default|SetCurrentTransitionA 0)
  (Variables|Default|SetCurrentTransitionB 0))

(event EventBeginPlay)

(event Collision|EventActorBeginOverlap
  (params (OtherActor :type Actor%20Object%20Reference)))

(event EventTick
  (params (DeltaSeconds :type Float%20%28single-precision%29)))

(fn ConstructionScript)

(fn BuildSoloTransition
  (params (DoorTransform :type Transform) (DoorTagType :type Gameplay%20Tag%20Structure))
  (LocalVariables|Setz DoorTagType)
  (LocalVariables|SetmFirstDoorTransform DoorTransform)
  (bind _returnvalue (Game|SpawnActorfromClass (.Value (Utilities|Map|Find (Variables|/Game/03-Game_Settings/Data/ProceduralMap/Transition/BDA_TransitionMap.BDA_TransitionMap_C|GetDoorTypeMapSolo (Variables|Default|GetTransitionMapping)) (LocalVariables|Getz))) (LocalVariables|GetmFirstDoorTransform) "Undefined" "MultiplyWithRoot" 0 0))
  (bind _output_get (Variables|Default|SetCurrentTransitionA _returnvalue))
  (bind _doesoverlap (CallFunction|CheckOverlap _output_get))
  (if _doesoverlap
    (return "" false true)
    (else
      (return (Transformation|GetWorldTransform (Variables|/Game/02_Blueprints/ProceduralMap/Transitions/BP_TransitionDoor.BP_TransitionDoor_C|GetAttachPointArrow _returnvalue)) (.ReturnValue (Utilities|Map|Find (Variables|/Game/03-Game_Settings/Data/ProceduralMap/Transition/BDA_TransitionMap.BDA_TransitionMap_C|GetDoorTypeMapSolo (Variables|Default|GetTransitionMapping)) (LocalVariables|Getz))) false))))

(fn BuildTransition
  (params (FirstDoorTransform :type Transform) (FirstDoorTypeTag :type Gameplay%20Tag%20Structure) (SecondDoorTypeTag :type Gameplay%20Tag%20Structure))
  (LocalVariables|SetNewLocalVar FirstDoorTypeTag)
  (LocalVariables|SetNewLocalVar_0 SecondDoorTypeTag)
  (LocalVariables|SetmFirstDoorTransform FirstDoorTransform)
  (bind _returnvalue (Game|SpawnActorfromClass (.Value (Utilities|Map|Find (Variables|/Game/03-Game_Settings/Data/ProceduralMap/Transition/BDA_TransitionMap.BDA_TransitionMap_C|GetDoorTypeMap (Variables|Default|GetTransitionMapping)) (LocalVariables|GetNewLocalVar))) (Math|Transform|MakeTransform "0.000000,0.000000,0.000000" "0, 0, 0" "1.000000,1.000000,1.000000") "Undefined" "MultiplyWithRoot" 0 0))
  (Variables|Default|SetCurrentTransitionA _returnvalue)
  (Transformation|SetActorTransform _returnvalue (Math|Transform|ComposeTransforms (Math|Transform|ComposeTransforms (Math|Transform|InvertTransform (Transformation|GetWorldTransform (Variables|/Game/02_Blueprints/ProceduralMap/Transitions/BP_TransitionDoor.BP_TransitionDoor_C|GetAttachPointArrow _returnvalue))) (Math|Transform|MakeTransform "0, 0, 0" "0.000000,180.000000,0.000000")) (LocalVariables|GetmFirstDoorTransform)))
  (bind _doesoverlap (CallFunction|CheckOverlap (Variables|Default|GetCurrentTransitionA)))
  (if _doesoverlap
    (return "" false true)
    (else
      (bind _returnvalue_2 (Game|SpawnActorfromClass (.Value (Utilities|Map|Find (Variables|/Game/03-Game_Settings/Data/ProceduralMap/Transition/BDA_TransitionMap.BDA_TransitionMap_C|GetDoorTypeMap (Variables|Default|GetTransitionMapping)) (LocalVariables|GetNewLocalVar_0))) (Math|Transform|ComposeTransforms (Math|Transform|MakeTransform "0, 0, 0" (Math|Rotator|MakeRotator 0.0 0.0 1.8e+02)) (Transformation|GetActorTransform _returnvalue)) "Undefined" "MultiplyWithRoot" 0 0))
      (bind _output_get (Variables|Default|SetCurrentTransitionB _returnvalue_2))
      (bind _doesoverlap_2 (CallFunction|CheckOverlap _output_get))
      (if _doesoverlap_2
        (return "" false true)
        (else
          (return (Transformation|GetWorldTransform (Variables|/Game/02_Blueprints/ProceduralMap/Transitions/BP_TransitionDoor.BP_TransitionDoor_C|GetAttachPointArrow _returnvalue_2)) (and (.ReturnValue (Utilities|Map|Find (Variables|/Game/03-Game_Settings/Data/ProceduralMap/Transition/BDA_TransitionMap.BDA_TransitionMap_C|GetDoorTypeMap (Variables|Default|GetTransitionMapping)) (LocalVariables|GetNewLocalVar))) (.ReturnValue (Utilities|Map|Find (Variables|/Game/03-Game_Settings/Data/ProceduralMap/Transition/BDA_TransitionMap.BDA_TransitionMap_C|GetDoorTypeMap (Variables|Default|GetTransitionMapping)) (LocalVariables|GetNewLocalVar_0)))) false))))))

(fn CheckOverlap
  (params (Transition :type BP%20Transition%20Door%20Object%20Reference))
  (bind _overlappingarray (LocalVariables|GetOverlappingArray))
  (LocalVariables|SetTransitionDoor Transition)
  (for _array_element (Components|GetChildrenComponents (Variables|/Game/02_Blueprints/ProceduralMap/Transitions/BP_TransitionDoor.BP_TransitionDoor_C|GetOverlappingComp Transition) false)
    (bind _asbox_collision (Utilities|Casting|CastToBoxComponent _array_element))
    (Utilities|Array|AppendArray (LocalVariables|GetOverlappingArray) (Class|PrimitiveComponent|GetOverlappingComponents _asbox_collision)))
  (if (Utilities|Array|IsEmpty _overlappingarray)
    (return false)
    (else
      (Development|PrintString (Utilities|GetDisplayName (Utilities|Array|Get(acopy) _overlappingarray)) true true "(R=0.308522,G=1.000000,B=0.217124,A=1.000000)" 3e+01)
      (return true))))