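; Simple command door for procedural map transitions that slides its single mesh upward when the player pawn overlaps its collision and lowers it when the player leaves.
; A timeline lerps the mesh from the position stored at BeginPlay to a raised offset, reversing to close.
; CaptureState saves the open flag in an instanced struct, and RestoreState replays the matching open or close path, both with debug prints.
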(event OnComponentBeginOverlap(Collision)
  (params (OverlappedComponent :type Primitive%20Component%20Object%20Reference) (OtherActor :type Actor%20Object%20Reference) (OtherComp :type Primitive%20Component%20Object%20Reference) (OtherBodyIndex :type Integer) (bFromSweep :type Boolean) (SweepResult :type Hit%20Result%20Structure%20%28by%20ref%29))
  (if (== OtherActor (Game|Player|GetPlayerPawn 0))
    (Variables|Default|SetOpen true)
    (bind _newtrack_0 (Timeline|Timeline Play)
      (:Update
        (Transformation|SetRelativeLocation (Variables|Default|GetSM_Door_L) (Math|Vector|Lerp(Vector) (Variables|Default|GetOriginalPosition) (+ (Variables|Default|GetOriginalPosition) "0.000000,0.000000,300.000000") _newtrack_0) false false)))))

(event OnComponentEndOverlap(Collision)
  (params (OverlappedComponent :type Primitive%20Component%20Object%20Reference) (OtherActor :type Actor%20Object%20Reference) (OtherComp :type Primitive%20Component%20Object%20Reference) (OtherBodyIndex :type Integer))
  (if (== OtherActor (Game|Player|GetPlayerPawn 0))
    (Variables|Default|SetOpen false)
    (bind _newtrack_0 (Timeline|Timeline Reverse)
      (:Update
        (Transformation|SetRelativeLocation (Variables|Default|GetSM_Door_L) (Math|Vector|Lerp(Vector) (Variables|Default|GetOriginalPosition) (+ (Variables|Default|GetOriginalPosition) "0.000000,0.000000,300.000000") _newtrack_0) false false)))))

(event EventBeginPlay
  (|CallParentFunction)
  (Variables|Default|SetOriginalPosition (Variables|/Script/Engine.SceneComponent|GetRelativeLocation (Variables|Default|GetSM_Door_L))))

(event Collision|EventActorBeginOverlap
  (params (OtherActor :type Actor%20Object%20Reference))
  (|CallParentFunction OtherActor) ; This node is disabled and will not be called.\nDrag off pins to build functionality.
)

(event EventTick
  (params (DeltaSeconds :type Float%20%28single-precision%29))
  (|CallParentFunction DeltaSeconds) ; This node is disabled and will not be called.\nDrag off pins to build functionality.
)

(event EventRestoreState
  (params (InState :type Instanced%20Struct%20Structure%20%28by%20ref%29))
  (bind _value (Utilities|InstancedStruct|GetInstancedStructValue InState)
    (:Valid
      (if (Utilities|Struct|BreakS_DoorDataSave _value)
        (Development|PrintString "HelloOpen")
        (Variables|Default|SetOpen true)
        (bind _newtrack_0 (Timeline|Timeline Play)
          (:Update
            (Transformation|SetRelativeLocation (Variables|Default|GetSM_Door_L) (Math|Vector|Lerp(Vector) (Variables|Default|GetOriginalPosition) (+ (Variables|Default|GetOriginalPosition) "0.000000,0.000000,300.000000") _newtrack_0) false false)))
        (else
          (Development|PrintString "HelloClose")
          (Variables|Default|SetOpen false)
          (Timeline|Timeline Reverse))))))

(fn ConstructionScript
  (|CallParentFunction))

(fn CaptureState
  (bind _returnvalue (Utilities|InstancedStruct|MakeInstancedStruct (Utilities|Struct|MakeS_DoorDataSave (Variables|Default|GetOpen))))
  (Development|PrintString "allg")
  (return _returnvalue))