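; BP_WoodenDoorSimple is a simple wooden door transition piece for the procedural map that removes its door mesh on overlap.
; When anything begins overlapping the Collision component, it prints that component's own name as red debug text, then destroys the SMDoorBStatic0 component if still valid.
; It has no filter on the overlapping actor, no animation and no logic to restore the door.
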(event OnComponentBeginOverlap(Collision)
  (params (OverlappedComponent :type Primitive%20Component%20Object%20Reference) (OtherActor :type Actor%20Object%20Reference) (OtherComp :type Primitive%20Component%20Object%20Reference) (OtherBodyIndex :type Integer) (bFromSweep :type Boolean) (SweepResult :type Hit%20Result%20Structure%20%28by%20ref%29))
  (Development|PrintString (Utilities|GetDisplayName OverlappedComponent) true true "(R=1.000000,G=0.089994,B=0.092859,A=1.000000)" 2e+01)
  (Variables|Default|GetSM_Door_B_Static_0
    (:then
      (Components|DestroyComponent (Variables|Default|GetSM_Door_B_Static_0)))
    (:else)))

(event EventBeginPlay
  (|CallParentFunction) ; This node is disabled and will not be called.\nDrag off pins to build functionality.
)

(event Collision|EventActorBeginOverlap
  (params (OtherActor :type Actor%20Object%20Reference))
  (|CallParentFunction OtherActor) ; This node is disabled and will not be called.\nDrag off pins to build functionality.
)

(event EventTick
  (params (DeltaSeconds :type Float%20%28single-precision%29))
  (|CallParentFunction DeltaSeconds) ; This node is disabled and will not be called.\nDrag off pins to build functionality.
)

(fn ConstructionScript
  (|CallParentFunction))