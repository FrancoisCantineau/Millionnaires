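; BP_ShortcutSpline is a procedural-map actor that draws a shortcut between two given world positions as an arrow-mesh spline.
; PlaceSpline clears the spline, rebuilds it from both positions, then adds a spline mesh component with a test arrow mesh for each point index looped over.
; Each mesh spans that index's world location to the next one's, with no tangents specified.
; Construction script and events are empty, so placement relies on calls to PlaceSpline.
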(event EventBeginPlay)

(event Collision|EventActorBeginOverlap
  (params (OtherActor :type Actor%20Object%20Reference)))

(event EventTick
  (params (DeltaSeconds :type Float%20%28single-precision%29)))

(fn ConstructionScript)

(fn PlaceSpline
  (params (PositionA :type Vector) (PositionB :type Vector))
  (bind _spline (Variables|Default|GetSpline))
  (Spline|ClearSplinePoints _spline true)
  (Spline|AddSplinePoint _spline PositionA "World" true)
  (Spline|AddSplinePoint _spline PositionB "World" true)
  (for _index (range 0 (Spline|GetNumberOfSplinePoints (Variables|Default|GetSpline)))
    (bind _returnvalue (AddComponent|AddSplineMeshComponent false))
    (Components|StaticMesh|SetStaticMesh _returnvalue "/Fab/Actors/GlobalFoliageActor/Geometry/Icon_Arrow_Test.Icon_Arrow_Test")
    (SplineMesh|SetStartandEnd _returnvalue (Spline|GetLocationatSplinePoint (Variables|Default|GetSpline) _index "World") "0, 0, 0" (Spline|GetLocationatSplinePoint (Variables|Default|GetSpline) (+ _index 1) "World") "0, 0, 0" true :!class /Script/Engine.SplineMeshComponent)))