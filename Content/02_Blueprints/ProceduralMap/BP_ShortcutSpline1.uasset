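; Spline actor that lays a repeated mesh along a path between two points, apparently as a shortcut in the procedural map.
; PlaceSpline rebuilds a four-point world-space spline, offsetting and orienting the middle points using each end's forward vector, then calls CustomEvent.
; CustomEvent and the construction script share a loop adding spline mesh segments every Fs units, with tangents clamped to that length; only CustomEvent makes them Movable.
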(event Custom|CustomEvent
  (for _index (range 0 (Math|Float|Truncate (/ (Spline|GetSplineLength (Variables|Default|GetSpline)) (Variables|Default|Getfs))))
    (Variables|Default|SetIndex _index)
    (bind _returnvalue (AddComponent|AddSplineMeshComponent false))
    (Transformation|SetMobility _returnvalue "Movable")
    (Components|StaticMesh|SetStaticMesh _returnvalue (Variables|Default|GetMesh))
    (SplineMesh|SetForwardAxis _returnvalue "Y" true)
    (bind (_newparam1 _newparam2) (CallFunction|GetStartPos (Variables|Default|GetIndex)))
    (bind (_newparam1_2 _newparam2_2) (CallFunction|GetEndPos (Variables|Default|GetIndex)))
    (SplineMesh|SetStartandEnd _returnvalue _newparam1 _newparam2 _newparam1_2 _newparam2_2 true :!class /Script/Engine.SplineMeshComponent)))

(event EventBeginPlay)

(event Collision|EventActorBeginOverlap
  (params (OtherActor :type Actor%20Object%20Reference)))

(event EventTick
  (params (DeltaSeconds :type Float%20%28single-precision%29)))

(fn ConstructionScript
  (for _index (range 0 (Math|Float|Truncate (/ (Spline|GetSplineLength (Variables|Default|GetSpline)) (Variables|Default|Getfs))))
    (Variables|Default|SetIndex _index)
    (bind _returnvalue (AddComponent|AddSplineMeshComponent false))
    (Components|StaticMesh|SetStaticMesh _returnvalue (Variables|Default|GetMesh))
    (SplineMesh|SetForwardAxis _returnvalue "Y" true)
    (bind (_newparam1 _newparam2) (CallFunction|GetStartPos (Variables|Default|GetIndex)))
    (bind (_newparam1_2 _newparam2_2) (CallFunction|GetEndPos (Variables|Default|GetIndex)))
    (SplineMesh|SetStartandEnd _returnvalue _newparam1 _newparam2 _newparam1_2 _newparam2_2 true :!class /Script/Engine.SplineMeshComponent)))

(fn PlaceSpline
  (params (PositionA :type Vector) (PositionB :type Vector) (TransformA :type Transform) (TransformB :type Transform) (NewParam :type Scene%20Component%20Object%20Reference) (NewParam1 :type Scene%20Component%20Object%20Reference))
  (bind _returnvalue (Math|Vector|GetForwardVector NewParam))
  (bind _returnvalue_2 (Math|Vector|GetForwardVector NewParam1))
  (bind _spline (Variables|Default|GetSpline))
  (Spline|ClearSplinePoints _spline true)
  (Spline|AddSplinePoint _spline PositionA "World" true)
  (Spline|AddSplinePoint _spline (+ PositionA (* _returnvalue 1e+02)) "World" true)
  (Spline|AddSplinePoint _spline (+ PositionB (* _returnvalue_2 1e+02)) "World" true)
  (Spline|AddSplinePoint _spline PositionB "World" true)
  (Spline|SetTangentatSplinePoint (Variables|Default|GetSpline) 1 (* _returnvalue 2e+01) "World" true)
  (Spline|SetTangentatSplinePoint (Variables|Default|GetSpline) 2 (- 1.0 (* _returnvalue_2 2e+01)) "World" true)
  (CallFunction|CustomEvent))

(fn GetStartPos
  (params (NewParam :type Integer))
  (bind _spline (Variables|Default|GetSpline))
  (bind _fs (Variables|Default|Getfs))
  (bind _returnvalue (* NewParam _fs))
  (return (Spline|GetLocationatDistanceAlongSpline _spline _returnvalue "Local") (Math|Vector|ClampVectorSize (Spline|GetTangentatDistanceAlongSpline _spline _returnvalue "Local") 0.0 (Variables|Default|Getfs))))

(fn GetEndPos
  (params (NewParam :type Integer))
  (bind _returnvalue (+ NewParam 1))
  (bind _spline (Variables|Default|GetSpline))
  (bind _fs (Variables|Default|Getfs))
  (bind _returnvalue_2 (* _returnvalue _fs))
  (return (Spline|GetLocationatDistanceAlongSpline _spline _returnvalue_2 "Local") (Math|Vector|ClampVectorSize (Spline|GetTangentatDistanceAlongSpline _spline _returnvalue_2 "Local") 0.0 (Variables|Default|Getfs))))