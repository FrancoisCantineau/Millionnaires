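; Weapon Blueprint that fires through an InstantAttackMode and uses the Gameplay Ability System for heat.
; CallAttack and a left mouse press both start the attack, while StopAttacking ends it.
; BeginPlay gives and activates the GA_HeatDecreasePassive ability once on the weapon's AbilitySystemComponent.
; Burst, charging and beam attack modes are referenced only by unused nodes.
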(event EventTick
  (params (DeltaSeconds :type Float%20%28single-precision%29)))

(event Collision|EventActorBeginOverlap
  (params (OtherActor :type Actor%20Object%20Reference)))

(event EventBeginPlay
  (Class|AbilitySystemComponent|GiveAbilityandActivateOnce (Variables|Default|GetAbilitySystemComponent) "/Game/02_Blueprints/GameplayAbilitySystem/Abilities/Weapons/GA_HeatDecreasePassive.GA_HeatDecreasePassive_C" 0 -1))

(event EventCallAttack
  (Class|AttackModeComponentBase|StartAttacking (Variables|Default|GetInstantAttackMode)))

(event EventStopAttacking
  (Class|AttackModeComponentBase|StopAttacking (Variables|Default|GetInstantAttackMode)))

(event Input|MouseEvents|LeftMouseButton
  (params (Key :type Key%20Structure :default "None"))
  (:Pressed
    (Class|AttackModeComponentBase|StartAttacking (Variables|Default|GetInstantAttackMode))))

(fn ConstructionScript)