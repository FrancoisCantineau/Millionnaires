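; BP_WeaponBase2 is a first-person weapon actor that pairs a beam attack component with a heat-based weapon component.
; On BeginPlay it switches the player mesh to the ABP_FP_Weapon animation class, attaches to the right-hand grip socket and takes the player pawn as owner.
; Left mouse or the Attack event starts BeamAttackMode, mouse release stops it, and R reloads HeatWeapon, using hard-coded key events.
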(event Collision|EventActorBeginOverlap
  (params (OtherActor :type Actor%20Object%20Reference)))

(event EventBeginPlay
  (bind _returnvalue (Game|GetPlayerCharacter 0))
  (bind _mesh (Variables|/Script/Engine.Character|GetMesh _returnvalue))
  (Components|SkeletalMesh|SetAnimInstanceClass _mesh "/Game/Variant_Shooter/Anims/ABP_FP_Weapon.ABP_FP_Weapon_C")
  (Transformation|AttachComponentToComponent _mesh "HandGrip_R" "SnapToTarget" "KeepRelative" "KeepWorld" true)
  (Actor|SetOwner (Game|Player|GetPlayerPawn 0)))

(event EventAttack
  (Class|AttackModeComponentBase|StartAttacking (Variables|Default|GetBeamAttackMode)))

(event Input|KeyboardEvents|R
  (params (Key :type Key%20Structure :default "None"))
  (:Pressed
    (Class|AmmoWeaponComponent|Reload (Variables|Default|GetHeatWeapon))))

(event Input|MouseEvents|LeftMouseButton
  (params (Key :type Key%20Structure :default "None"))
  (bind _beamattackmode (Variables|Default|GetBeamAttackMode))
  (:Pressed
    (Class|AttackModeComponentBase|StartAttacking _beamattackmode))
  (:Released
    (Class|AttackModeComponentBase|StopAttacking _beamattackmode)))

(fn ConstructionScript)