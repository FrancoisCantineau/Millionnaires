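; Base weapon actor that equips itself on the first player and handles attacking and reloading.
; On BeginPlay it switches the player mesh to the first-person weapon anim class, snaps onto its right-hand socket and takes the pawn as owner.
; CallAttack or left mouse starts InstantAttackMode, StopAttacking ends it, and R reloads through AmmoWeapon.
; Burst, charging and beam modes and ability-system attribute reads are left unwired.
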(event EventStopAttacking
  (Class|AttackModeComponentBase|StopAttacking (Variables|Default|GetInstantAttackMode)))

(event Collision|EventActorBeginOverlap
  (params (OtherActor :type Actor%20Object%20Reference)))

(event EventBeginPlay
  (bind _returnvalue (Game|GetPlayerCharacter 0))
  (bind _mesh (Variables|/Script/Engine.Character|GetMesh _returnvalue))
  (Components|SkeletalMesh|SetAnimInstanceClass _mesh "/Game/Variant_Shooter/Anims/ABP_FP_Weapon.ABP_FP_Weapon_C")
  (Transformation|AttachComponentToComponent _mesh "HandGrip_R" "SnapToTarget" "SnapToTarget" "KeepWorld" true)
  (Actor|SetOwner (Game|Player|GetPlayerPawn 0)))

(event EventCallAttack
  (Class|AttackModeComponentBase|StartAttacking (Variables|Default|GetInstantAttackMode)))

(event EventTick
  (params (DeltaSeconds :type Float%20%28single-precision%29)))

(event Input|KeyboardEvents|R
  (params (Key :type Key%20Structure :default "None"))
  (:Pressed
    (Class|AmmoWeaponComponent|Reload (Variables|Default|GetAmmoWeapon))))

(event Input|MouseEvents|LeftMouseButton
  (params (Key :type Key%20Structure :default "None"))
  (:Pressed
    (Class|AttackModeComponentBase|StartAttacking (Variables|Default|GetInstantAttackMode))))

(fn ConstructionScript)