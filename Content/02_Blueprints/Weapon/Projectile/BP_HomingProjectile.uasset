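; BP_HomingProjectile is a weapon projectile that locks onto a nearby pawn and homes in on it.
; Until a target is found, each Tick runs a sphere overlap around the mesh for Pawns, ignoring the first player's pawn.
; The nearest hit's root component becomes the ProjectileMovement homing target, and FoundTarget stops further searches, so the lock never changes.
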(event EventBeginPlay)

(event Collision|EventActorBeginOverlap
  (params (OtherActor :type Actor%20Object%20Reference)))

(event EventTick
  (params (DeltaSeconds :type Float%20%28single-precision%29))
  (if (not (Variables|Default|GetFoundTarget))
    (bind (_outactors _returnvalue) (Collision|SphereOverlapActors (Transformation|GetWorldLocation (Variables|Default|GetMeshComponent)) 3e+02 (Utilities|Array|MakeArray "ObjectTypeQuery3") 0 (Utilities|Array|MakeArray (Game|Player|GetPlayerPawn 0))))
    (if _returnvalue
      (Variables|Default|SetFoundTarget true)
      (Variables|/Script/Engine.ProjectileMovementComponent|SetHomingTargetComponent (Variables|Default|GetProjectileMovement) (Variables|/Script/Engine.Actor|GetRootComponent (.ReturnValue (Actor|FindNearestActor (Transformation|GetWorldLocation (Variables|Default|GetMeshComponent)) _outactors)))))))

(fn ConstructionScript)