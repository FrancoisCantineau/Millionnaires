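; BP_GlobalSaveTest is a test actor for the global save system, persisting a counter across save and restore.
; On BeginPlay it registers itself with GlobalSaveableRegistrySubsystem under the "Increment" key.
; CaptureState prints the counter and returns it wrapped in an SIncrementTest instanced struct.
; RestoreState unpacks that struct, prints the saved value and stores it plus one, so the count grows with each restore.
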(event EventBeginPlay
  (Class|GlobalSaveableRegistrySubsystem|RegisterGlobalSaveable (Subsystems|GetGlobalSaveableRegistrySubsystem) "Increment" self))

(event Collision|EventActorBeginOverlap
  (params (OtherActor :type Actor%20Object%20Reference)))

(event EventTick
  (params (DeltaSeconds :type Float%20%28single-precision%29)))

(event EventRestoreState
  (params (InState :type Instanced%20Struct%20Structure%20%28by%20ref%29))
  (bind _value (Utilities|InstancedStruct|GetInstancedStructValue InState)
    (:Valid
      (Development|PrintString (Utilities|String|ToString(Integer) (Utilities|Struct|BreakS_IncrementTest _value)))
      (Variables|Default|SetcounterTest (+ (Utilities|Struct|BreakS_IncrementTest _value) 1)))))

(fn ConstructionScript)

(fn CaptureState
  (Development|PrintString (Utilities|String|ToString(Integer) (Variables|Default|GetcounterTest)))
  (bind _returnvalue (Utilities|InstancedStruct|MakeInstancedStruct (Utilities|Struct|MakeS_IncrementTest (Variables|Default|GetcounterTest))))
  (return _returnvalue))