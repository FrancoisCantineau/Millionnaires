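; Test player character Blueprint that drives Gameplay Ability System weapon features from hard-coded debug keys.
; Keys spawn a test melee or heat weapon into a shared variable, then send equip gameplay events carrying it with a wrench or rifle tag.
; Other keys activate reload, attack and attack-rate abilities by class, and psychose regen by tag.
; Attribute printing, spotlight and ability-granting snippets are left unconnected.
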(event Collision|EventActorBeginOverlap
  (params (OtherActor :type Actor%20Object%20Reference)))

(event EventTick
  (params (DeltaSeconds :type Float%20%28single-precision%29)))

(event EventBeginPlay)

(event Input|KeyboardEvents|B
  (params (Key :type Key%20Structure :default "None"))
  (:Pressed
    (Abilities|TryActivateAbilitybyClass (Variables|Default|GetAbilitySystemComponent) "/Game/02_Blueprints/GameplayAbilitySystem/Abilities/Weapons/GA_ModifyAttackRate.GA_ModifyAttackRate_C" true)))

(event Input|KeyboardEvents|V
  (params (Key :type Key%20Structure :default "None"))
  (:Pressed
    (Abilities|TryActivateAbilitybyClass (Variables|Default|GetAbilitySystemComponent) "/Game/02_Blueprints/GameplayAbilitySystem/Abilities/Weapons/GA_WeaponReload.GA_WeaponReload_C" true)))

(event Input|KeyboardEvents|T
  (params (Key :type Key%20Structure :default "None"))
  (:Pressed
    (Abilities|TryActivateAbilitybyClass (Variables|Default|GetAbilitySystemComponent) "/Game/02_Blueprints/GameplayAbilitySystem/Abilities/Weapons/GA_WeaponAttack.GA_WeaponAttack_C" true))
  (:Released
    (Class|AbilitySystemComponent|ReleaseInputID (Variables|Default|GetAbilitySystemComponent) 1)))

(event Input|KeyboardEvents|C
  (params (Key :type Key%20Structure :default "None"))
  (:Pressed
    (bind _returnvalue (Game|SpawnActorfromClass "/Game/02_Blueprints/Weapon/BP_WeaponHeat.BP_WeaponHeat_C" (Math|Transform|MakeTransform "0, 0, 0" "0, 0, 0" "1.000000,1.000000,1.000000") "AlwaysSpawn" "MultiplyWithRoot" 0 0))
    (Variables|Default|SetNewVar _returnvalue)))

(event Input|KeyboardEvents|N
  (params (Key :type Key%20Structure :default "None"))
  (:Pressed
    (Abilities|TryActivateAbilitiesbyTag (Variables|Default|GetAbilitySystemComponent) (GameplayTags|MakeGameplayTagContainerfromTag "(TagName=\"GameplayAbility.Regen.Psychose\")") true)))

(event Input|KeyboardEvents|F
  (params (Key :type Key%20Structure :default "None")))

(event Input|KeyboardEvents|J
  (params (Key :type Key%20Structure :default "None"))
  (:Pressed
    (Ability|SendGameplayEventtoActor self "(TagName=\"Event.Weapon.Equip\")" (Utilities|Struct|MakeGameplayEventData (Variables|Default|GetNewVar) "(GameplayTags=((TagName=\"Weapon.Range.Rifle\")))"))))

(event Input|KeyboardEvents|X
  (params (Key :type Key%20Structure :default "None"))
  (:Pressed
    (bind _returnvalue (Game|SpawnActorfromClass "/Game/02_Blueprints/Weapon/BP_MeleeWeaponTest.BP_MeleeWeaponTest_C" (Math|Transform|MakeTransform "0, 0, 0" "0, 0, 0" "1.000000,1.000000,1.000000") "AlwaysSpawn" "MultiplyWithRoot" 0 0))
    (Variables|Default|SetNewVar _returnvalue)))

(event Input|KeyboardEvents|K
  (params (Key :type Key%20Structure :default "None"))
  (:Pressed
    (Ability|SendGameplayEventtoActor self "(TagName=\"Event.Weapon.Equip\")" (Utilities|Struct|MakeGameplayEventData (Variables|Default|GetNewVar) "(GameplayTags=((TagName=\"Weapon.Melee.Wrench\")))"))))

(fn ConstructionScript)