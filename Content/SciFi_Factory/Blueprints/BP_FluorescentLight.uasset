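; Fluorescent light fixture with three tube meshes and a rect light that periodically flickers.
; Construction script applies exposed light settings and tube emissive values; BeginPlay reapplies emissive and sets the tube base color.
; BeginPlay also starts a looping Pulse timer, its interval randomized once within a set range.
; Each Pulse runs timelines driving light intensity and one random tube's emissive, restoring configured values when finished.
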(event Custom|Pulse
  (bind _rectlight (Variables|Default|GetRectLight))
  (Utilities|FlowControl|Sequence
    (:then_0
      (bind _newtrack_0 (Timeline|Timeline PlayFromStart)
        (:Update
          (Rendering|Components|Light|SetIntensity _rectlight _newtrack_0))
        (:Finished
          (Rendering|Components|Light|SetIntensity _rectlight (Variables|Default|GetLightINtensity)))))
    (:then_1
      (Variables|Default|SetWhichLight? (Math|Random|RandomIntegerinRange 0 2))
      (bind _newtrack_0_2 (Timeline|LightPulse PlayFromStart)
        (:Update
          (Rendering|Material|SetScalarParameterValueonMaterials (Utilities|Select :Index (Variables|Default|GetWhichLight?) :Option%200 (Variables|Default|GetMesh_FluorescentLight) :Option%201 (Variables|Default|GetMesh_FluorescentLight1) :Option%202 (Variables|Default|GetMesh_FluorescentLight2)) "Emissive" _newtrack_0_2))
        (:Finished
          (Rendering|Material|SetScalarParameterValueonMaterials (Utilities|Select :Index (Variables|Default|GetWhichLight?) :Option%200 (Variables|Default|GetMesh_FluorescentLight) :Option%201 (Variables|Default|GetMesh_FluorescentLight1) :Option%202 (Variables|Default|GetMesh_FluorescentLight2)) "Emissive" (Variables|Default|GetLight_Emissive)))))))

(event EventBeginPlay
  (Rendering|Material|SetScalarParameterValueonMaterials (Variables|Default|GetMesh_FluorescentLight) "Emissive" (Variables|Default|GetLight_Emissive))
  (bind _returnvalue (Rendering|Material|CreateDynamicMaterialInstance (Variables|Default|GetMesh_FluorescentLight) 0 0 "None" :!class /Script/Engine.PrimitiveComponent))
  (Rendering|Material|SetVectorParameterValue _returnvalue "Emissive Color" (Variables|Default|GetEmissiveColor) :!class /Script/Engine.MaterialInstanceDynamic)
  (Rendering|Material|SetVectorParameterValue _returnvalue "Color" (Variables|Default|GetTurnOffColor) :!class /Script/Engine.MaterialInstanceDynamic)
  (Rendering|Material|SetScalarParameterValueonMaterials (Variables|Default|GetMesh_FluorescentLight1) "Emissive" (Variables|Default|GetLight_Emissive))
  (bind _returnvalue_2 (Rendering|Material|CreateDynamicMaterialInstance (Variables|Default|GetMesh_FluorescentLight1) 0 0 "None" :!class /Script/Engine.PrimitiveComponent))
  (Rendering|Material|SetVectorParameterValue _returnvalue_2 "Emissive Color" (Variables|Default|GetEmissiveColor) :!class /Script/Engine.MaterialInstanceDynamic)
  (Rendering|Material|SetVectorParameterValue _returnvalue_2 "Color" (Variables|Default|GetTurnOffColor) :!class /Script/Engine.MaterialInstanceDynamic)
  (Rendering|Material|SetScalarParameterValueonMaterials (Variables|Default|GetMesh_FluorescentLight2) "Emissive" (Variables|Default|GetLight_Emissive))
  (bind _returnvalue_3 (Rendering|Material|CreateDynamicMaterialInstance (Variables|Default|GetMesh_FluorescentLight2) 0 0 "None" :!class /Script/Engine.PrimitiveComponent))
  (Rendering|Material|SetVectorParameterValue _returnvalue_3 "Emissive Color" (Variables|Default|GetEmissiveColor) :!class /Script/Engine.MaterialInstanceDynamic)
  (Rendering|Material|SetVectorParameterValue _returnvalue_3 "Color" (Variables|Default|GetTurnOffColor) :!class /Script/Engine.MaterialInstanceDynamic)
  (Utilities|Time|SetTimerbyFunctionName 0 "Pulse" (Math|Conversions|ToFloat(Integer) (Math|Random|RandomIntegerinRange (Variables|Default|GetMinRandom) (Variables|Default|GetMaxRandom))) true))

(event Collision|EventActorBeginOverlap
  (params (OtherActor :type Actor%20Object%20Reference)))

(event EventTick
  (params (DeltaSeconds :type Float%20%28single-precision%29)))

(fn ConstructionScript
  (bind _rectlight (Variables|Default|GetRectLight))
  (Rendering|Material|SetScalarParameterValueonMaterials (Variables|Default|GetMesh_FluorescentLight) "Emissive" (Variables|Default|GetLight_Emissive))
  (bind _returnvalue (Rendering|Material|CreateDynamicMaterialInstance (Variables|Default|GetMesh_FluorescentLight) 0 0 "None" :!class /Script/Engine.PrimitiveComponent))
  (Rendering|Material|SetVectorParameterValue _returnvalue "Emissive Color" (Variables|Default|GetEmissiveColor) :!class /Script/Engine.MaterialInstanceDynamic)
  (Rendering|Material|SetScalarParameterValueonMaterials (Variables|Default|GetMesh_FluorescentLight1) "Emissive" (Variables|Default|GetLight_Emissive))
  (bind _returnvalue_2 (Rendering|Material|CreateDynamicMaterialInstance (Variables|Default|GetMesh_FluorescentLight1) 0 0 "None" :!class /Script/Engine.PrimitiveComponent))
  (Rendering|Material|SetVectorParameterValue _returnvalue_2 "Emissive Color" (Variables|Default|GetEmissiveColor) :!class /Script/Engine.MaterialInstanceDynamic)
  (Rendering|Material|SetScalarParameterValueonMaterials (Variables|Default|GetMesh_FluorescentLight2) "Emissive" (Variables|Default|GetLight_Emissive))
  (bind _returnvalue_3 (Rendering|Material|CreateDynamicMaterialInstance (Variables|Default|GetMesh_FluorescentLight2) 0 0 "None" :!class /Script/Engine.PrimitiveComponent))
  (Rendering|Material|SetVectorParameterValue _returnvalue_3 "Emissive Color" (Variables|Default|GetEmissiveColor) :!class /Script/Engine.MaterialInstanceDynamic)
  (Rendering|Components|Light|SetIntensity _rectlight (Variables|Default|GetLightINtensity))
  (Rendering|Components|Light|SetLightColor _rectlight (Variables|Default|GetLightColor) true)
  (Class|LightComponent|SetTemperature _rectlight (Variables|Default|GetLightTemperature))
  (Class|LightComponent|SetIndirectLightingIntensity _rectlight (Variables|Default|GetLightINdirectIntensity))
  (Rendering|Lighting|SetAttenuationRadius _rectlight (Variables|Default|GetLightAttenuation)))