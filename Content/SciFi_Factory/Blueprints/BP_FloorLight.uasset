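; BP_FloorLight is a configurable floor lamp prop with a rect light and emissive mesh that periodically pulses.
; The construction script applies tilt and swivel offsets to the head and leg, plus light and material settings.
; BeginPlay creates a dynamic material and starts a looping Pulse timer with a random integer interval picked once.
; Pulse runs two timelines in parallel, animating light intensity and emissive strength, then restoring configured values.
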(event Custom|Pulse
  (bind _rectlight (Variables|Default|GetRectLight))
  (bind _sm_floorlight_light (Variables|Default|GetSM_FloorLight_Light))
  (Utilities|FlowControl|Sequence
    (:then_0
      (bind _newtrack_0 (Timeline|Timeline PlayFromStart)
        (:Update
          (Rendering|Components|Light|SetIntensity _rectlight _newtrack_0))
        (:Finished
          (Rendering|Components|Light|SetIntensity _rectlight (Variables|Default|GetLightINtensity)))))
    (:then_1
      (bind _newtrack_0_2 (Timeline|LightPulse PlayFromStart)
        (:Update
          (Rendering|Material|SetScalarParameterValueonMaterials _sm_floorlight_light "Emissive" _newtrack_0_2))
        (:Finished
          (Rendering|Material|SetScalarParameterValueonMaterials _sm_floorlight_light "Emissive" (Variables|Default|GetLight_Emissive)))))))

(event EventBeginPlay
  (bind _returnvalue (Rendering|Material|CreateDynamicMaterialInstance (Variables|Default|GetSM_FloorLight_Light) 5 (Variables|Default|GetEmissiveMaterial) "None" :!class /Script/Engine.PrimitiveComponent))
  (Rendering|Material|SetVectorParameterValue _returnvalue "Emissive Color" (Variables|Default|GetEmissiveColor) :!class /Script/Engine.MaterialInstanceDynamic)
  (Rendering|Material|SetVectorParameterValue _returnvalue "Color" (Variables|Default|GetTurnOffColor) :!class /Script/Engine.MaterialInstanceDynamic)
  (Rendering|Material|SetScalarParameterValue _returnvalue "Emissive" (Variables|Default|GetLight_Emissive) :!class /Script/Engine.MaterialInstanceDynamic)
  (Utilities|Time|SetTimerbyFunctionName 0 "Pulse" (Math|Conversions|ToFloat(Integer) (Math|Random|RandomIntegerinRange (Variables|Default|GetMinRandom) (Variables|Default|GetMaxRandom))) true))

(event Collision|EventActorBeginOverlap
  (params (OtherActor :type Actor%20Object%20Reference)))

(event EventTick
  (params (DeltaSeconds :type Float%20%28single-precision%29)))

(fn ConstructionScript
  (bind _sm_floorlight_light (Variables|Default|GetSM_FloorLight_Light))
  (bind _emissivematerial (Variables|Default|GetEmissiveMaterial))
  (bind _light_emissive (Variables|Default|GetLight_Emissive))
  (bind _rectlight (Variables|Default|GetRectLight))
  (Transformation|SetRelativeRotation (Variables|Default|GetSM_FloorLight_Light) (Math|Rotator|MakeRotator 0.0 (+ (.pitch (Variables|/Script/Engine.SceneComponent|GetRelativeRotation (Variables|Default|GetSM_FloorLight_Light))) (Math|Float|Clamp(Float) (Math|Conversions|ToFloat(Integer) (Variables|Default|GetUpDown)) -1e+01 2e+02)) 0.0) false false)
  (Transformation|SetRelativeRotation (Variables|Default|GetSM_FloorLight_Leg) (Math|Rotator|MakeRotator 0.0 0.0 (+ (.pitch (Variables|/Script/Engine.SceneComponent|GetRelativeRotation (Variables|Default|GetSM_FloorLight_Leg))) (Variables|Default|GetRightLeft))) false false)
  (Rendering|Material|SetMaterialbyName _sm_floorlight_light "Light" _emissivematerial)
  (Rendering|Material|SetScalarParameterValueonMaterials _sm_floorlight_light "Emissive" _light_emissive)
  (bind _returnvalue (Rendering|Material|CreateDynamicMaterialInstance _sm_floorlight_light 5 _emissivematerial "" :!class /Script/Engine.PrimitiveComponent))
  (Rendering|Material|SetVectorParameterValue _returnvalue "Emissive Color" (Variables|Default|GetEmissiveColor) :!class /Script/Engine.MaterialInstanceDynamic)
  (Rendering|Material|SetScalarParameterValue _returnvalue "Emissive" _light_emissive :!class /Script/Engine.MaterialInstanceDynamic)
  (Rendering|Components|Light|SetIntensity _rectlight (Variables|Default|GetLightINtensity))
  (Rendering|Components|Light|SetLightColor _rectlight (Variables|Default|GetLightColor) true)
  (Class|LightComponent|SetTemperature _rectlight (Variables|Default|GetLightTemperature))
  (Class|LightComponent|SetIndirectLightingIntensity _rectlight (Variables|Default|GetLightINdirectIntensity))
  (Rendering|Lighting|SetAttenuationRadius _rectlight (Variables|Default|GetLightAttenuation)))