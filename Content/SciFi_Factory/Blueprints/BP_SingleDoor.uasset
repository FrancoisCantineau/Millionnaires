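; Interactive sci-fi single door that swings open away from or toward either side and doubles as a level-streaming trigger.
; Front/back proximity boxes enable input and raise prompt widgets; the action key plays side-specific open/close animations, unless locked.
; Two level volumes load their streamed levels on entry, then auto-close the door and conditionally unload on exit, suppressed inside the DontCloseDoor volume.
; The construction script applies door color and locked-state widgets.
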(event OnComponentBeginOverlap(BoxProxy_Front)
  (params (OverlappedComponent :type Primitive%20Component%20Object%20Reference) (OtherActor :type Actor%20Object%20Reference) (OtherComp :type Primitive%20Component%20Object%20Reference) (OtherBodyIndex :type Integer) (bFromSweep :type Boolean) (SweepResult :type Hit%20Result%20Structure%20%28by%20ref%29))
  ;[1 1 1] Start Overlap&End
  (Utilities|Casting|CastToBP_FirstPersonCharacter OtherActor)
  (Input|EnableInput (Game|GetPlayerController 0))
  (Variables|Default|SetWhichSide? "Front")
  (CallFunction|GoUp))

(event OnComponentEndOverlap(BoxProxy_Front)
  (params (OverlappedComponent :type Primitive%20Component%20Object%20Reference) (OtherActor :type Actor%20Object%20Reference) (OtherComp :type Primitive%20Component%20Object%20Reference) (OtherBodyIndex :type Integer))
  ;[1 1 1] Start Overlap&End
  (Utilities|Casting|CastToBP_FirstPersonCharacter OtherActor)
  (Input|DisableInput (Game|GetPlayerController 0))
  (Variables|Default|SetWhichSide? "none")
  (CallFunction|GoDown))

(event OnComponentEndOverlap(NextLvl_1)
  (params (OverlappedComponent :type Primitive%20Component%20Object%20Reference) (OtherActor :type Actor%20Object%20Reference) (OtherComp :type Primitive%20Component%20Object%20Reference) (OtherBodyIndex :type Integer))
  ;[1 1 1] Next Level
  (CallFunction|ClosetheDoor)
  (Variables|Default|SetUnload? true)
  (Variables|Default|SetI%20am%20in%20NextLvl false)
  (if (or (== (Variables|Default|GetI%20am%20in%20CurrentLvl) (Variables|Default|GetI%20am%20in%20NextLvl)) (== (Variables|Default|GetDontCloseDoor?) false))
    (if (and (== (Variables|Default|GetUnload?) true) (== (Variables|Default|GetDontCloseDoor?) false))
      (Game|UnloadStreamLevel(byName) (Utilities|String|StringToName (Utilities|Select :Index (Variables|Default|GetWhereAreU?) :Option%200 (Utilities|String|ToString(Name) (Variables|Default|GetLevelToLoad)) :Option%201 (Utilities|String|ToString(Name) (Variables|Default|GetLevelTOUnload)))) false))))

(event OnComponentEndOverlap(CurrentLvl_0)
  (params (OverlappedComponent :type Primitive%20Component%20Object%20Reference) (OtherActor :type Actor%20Object%20Reference) (OtherComp :type Primitive%20Component%20Object%20Reference) (OtherBodyIndex :type Integer))
  ;[1 1 1] Current Level
  (CallFunction|ClosetheDoor)
  (Variables|Default|SetUnload? true)
  (Variables|Default|SetI%20am%20in%20CurrentLvl false)
  (if (or (== (Variables|Default|GetI%20am%20in%20CurrentLvl) (Variables|Default|GetI%20am%20in%20NextLvl)) (== (Variables|Default|GetDontCloseDoor?) false))
    (if (and (== (Variables|Default|GetUnload?) true) (== (Variables|Default|GetDontCloseDoor?) false))
      (Game|UnloadStreamLevel(byName) (Utilities|String|StringToName (Utilities|Select :Index (Variables|Default|GetWhereAreU?) :Option%200 (Utilities|String|ToString(Name) (Variables|Default|GetLevelToLoad)) :Option%201 (Utilities|String|ToString(Name) (Variables|Default|GetLevelTOUnload)))) false))))

(event OnComponentBeginOverlap(BoxProxy_Back)
  (params (OverlappedComponent :type Primitive%20Component%20Object%20Reference) (OtherActor :type Actor%20Object%20Reference) (OtherComp :type Primitive%20Component%20Object%20Reference) (OtherBodyIndex :type Integer) (bFromSweep :type Boolean) (SweepResult :type Hit%20Result%20Structure%20%28by%20ref%29))
  ;[1 1 1] Start Overlap&End
  (Utilities|Casting|CastToBP_FirstPersonCharacter OtherActor)
  (Input|EnableInput (Game|GetPlayerController 0))
  (Variables|Default|SetWhichSide? "Back")
  (CallFunction|GoUp))

(event OnComponentEndOverlap(BoxProxy_Back)
  (params (OverlappedComponent :type Primitive%20Component%20Object%20Reference) (OtherActor :type Actor%20Object%20Reference) (OtherComp :type Primitive%20Component%20Object%20Reference) (OtherBodyIndex :type Integer))
  ;[1 1 1] Start Overlap&End
  (Utilities|Casting|CastToBP_FirstPersonCharacter OtherActor)
  (Input|DisableInput (Game|GetPlayerController 0))
  (Variables|Default|SetWhichSide? "none")
  (CallFunction|GoDown))

(event OnComponentBeginOverlap(CurrentLvl_0)
  (params (OverlappedComponent :type Primitive%20Component%20Object%20Reference) (OtherActor :type Actor%20Object%20Reference) (OtherComp :type Primitive%20Component%20Object%20Reference) (OtherBodyIndex :type Integer) (bFromSweep :type Boolean) (SweepResult :type Hit%20Result%20Structure%20%28by%20ref%29))
  ;[1 1 1] Current Level
  (Variables|Default|SetUnload? false)
  (Variables|Default|SetWhereAreU? 0)
  (Variables|Default|SetI%20am%20in%20CurrentLvl true)
  (Game|LoadStreamLevel(byName) (Variables|Default|GetLevelToLoad) true)
  (Default|CallLoadingLvlSingleDoor))

(event OnComponentBeginOverlap(NextLvl_1)
  (params (OverlappedComponent :type Primitive%20Component%20Object%20Reference) (OtherActor :type Actor%20Object%20Reference) (OtherComp :type Primitive%20Component%20Object%20Reference) (OtherBodyIndex :type Integer) (bFromSweep :type Boolean) (SweepResult :type Hit%20Result%20Structure%20%28by%20ref%29))
  ;[1 1 1] Next Level
  (Variables|Default|SetUnload? false)
  (Variables|Default|SetWhereAreU? 1)
  (Variables|Default|SetI%20am%20in%20NextLvl true)
  (Game|LoadStreamLevel(byName) (Variables|Default|GetLevelTOUnload) true)
  (Default|CallLoadingLvlSingleDoor))

(event OnComponentBeginOverlap(DontCloseDoor)
  (params (OverlappedComponent :type Primitive%20Component%20Object%20Reference) (OtherActor :type Actor%20Object%20Reference) (OtherComp :type Primitive%20Component%20Object%20Reference) (OtherBodyIndex :type Integer) (bFromSweep :type Boolean) (SweepResult :type Hit%20Result%20Structure%20%28by%20ref%29))
  ;[1 1 1] Dont Close the door
  (Variables|Default|SetDontCloseDoor? true)
  (Variables|Default|SetUnload? false))

(event OnComponentEndOverlap(DontCloseDoor)
  (params (OverlappedComponent :type Primitive%20Component%20Object%20Reference) (OtherActor :type Actor%20Object%20Reference) (OtherComp :type Primitive%20Component%20Object%20Reference) (OtherBodyIndex :type Integer))
  ;[1 1 1] Dont Close the door
  (Variables|Default|SetDontCloseDoor? false)
  (Variables|Default|SetUnload? false))

(event Custom|GoDown
  ;[1 1 1] Transfer Widget
  (bind _newtrack_0 (Timeline|Anim_GoUp Reverse)
    (:Update
      (Transformation|SetRelativeLocation (Variables|Default|GetWidget_Body_Front) (Math|Vector|MakeVector 22.866173 -9.067741 (.z _newtrack_0)) false false)
      (Transformation|SetRelativeLocation (Variables|Default|GetWidget_Body_Back) (Math|Vector|MakeVector 13.636892 2.78419 (.z _newtrack_0)) false false))))

(event Custom|GoUp
  ;[1 1 1] Transfer Widget
  (bind _newtrack_0 (Timeline|Anim_GoUp Play)
    (:Update
      (Transformation|SetRelativeLocation (Variables|Default|GetWidget_Body_Front) (Math|Vector|MakeVector 22.866173 -9.067741 (.z _newtrack_0)) false false)
      (Transformation|SetRelativeLocation (Variables|Default|GetWidget_Body_Back) (Math|Vector|MakeVector 13.636892 2.78419 (.z _newtrack_0)) false false))))

(event EventBeginPlay)

(event Collision|EventActorBeginOverlap
  (params (OtherActor :type Actor%20Object%20Reference)))

(event EventTick
  (params (DeltaSeconds :type Float%20%28single-precision%29)))

(event Input|ActionEvents|InputActionAction
  (params (Key :type Key%20Structure))
  ;[1 1 1] Open and Close the door
  (:Pressed
    (if (not (Variables|Default|GetIsLocked?))
      (if (Utilities|Enum|Equal(Enum) (Variables|Default|GetWhichSide?) "Front")
        (if (Utilities|Enum|Equal(Enum) (Variables|Default|GetWhichSideOpened?) "Closed")
          (Utilities|FlowControl|DoOnce false :!label _label
            (:Completed
              (Components|Animation|PlayAnimation (Variables|Default|GetSKM_SingleDoor_Animated) "/Game/SciFi_Factory/SkeletonMeshes/SKM_SingleDoor_Open_Front.SKM_SingleDoor_Open_Front" false)
              (Rendering|SetVisibility (Variables|Default|GetWidget_Line_Front) false false)
              (Variables|Default|SetWhichSideOpened? "Front")
              (Utilities|FlowControl|Delay 1.0)
              (goto _label Reset)))
          (elif (Utilities|Enum|Equal(Enum) (Variables|Default|GetWhichSideOpened?) "Front")
            (Utilities|FlowControl|DoOnce false :!label _label_2
              (:Completed
                (Components|Animation|PlayAnimation (Variables|Default|GetSKM_SingleDoor_Animated) "/Game/SciFi_Factory/SkeletonMeshes/SKM_SingleDoor_Close_Front.SKM_SingleDoor_Close_Front" false)
                (Variables|Default|SetWhichSideOpened? "Closed")
                (Utilities|FlowControl|Delay 1.0)
                (Rendering|SetVisibility (Variables|Default|GetWidget_Line_Front) true false)
                (goto _label_2 Reset)))
            (else
              (Utilities|FlowControl|DoOnce false :!label _label_3
                (:Completed
                  (Components|Animation|PlayAnimation (Variables|Default|GetSKM_SingleDoor_Animated) "/Game/SciFi_Factory/SkeletonMeshes/SKM_SingleDoor_Close_Back.SKM_SingleDoor_Close_Back" false)
                  (Variables|Default|SetWhichSideOpened? "Closed")
                  (Utilities|FlowControl|Delay 1.0)
                  (Rendering|SetVisibility (Variables|Default|GetWidget_Line_Front) true false)
                  (goto _label_3 Reset))))))
        (elif (Utilities|Enum|Equal(Enum) (Variables|Default|GetWhichSideOpened?) "Closed")
          (Utilities|FlowControl|DoOnce false :!label _label_4
            (:Completed
              (Components|Animation|PlayAnimation (Variables|Default|GetSKM_SingleDoor_Animated) "/Game/SciFi_Factory/SkeletonMeshes/SKM_SingleDoor_Open_Back.SKM_SingleDoor_Open_Back" false)
              (Rendering|SetVisibility (Variables|Default|GetWidget_Line_Front) false false)
              (Variables|Default|SetWhichSideOpened? "Back")
              (Utilities|FlowControl|Delay 1.0)
              (goto _label_4 Reset)))
          (elif (Utilities|Enum|Equal(Enum) (Variables|Default|GetWhichSideOpened?) "Back")
            (Utilities|FlowControl|DoOnce false :!label _label_5
              (:Completed
                (Components|Animation|PlayAnimation (Variables|Default|GetSKM_SingleDoor_Animated) "/Game/SciFi_Factory/SkeletonMeshes/SKM_SingleDoor_Close_Back.SKM_SingleDoor_Close_Back" false)
                (Variables|Default|SetWhichSideOpened? "Closed")
                (Utilities|FlowControl|Delay 1.0)
                (Rendering|SetVisibility (Variables|Default|GetWidget_Line_Front) true false)
                (goto _label_5 Reset)))
            (else
              (Utilities|FlowControl|DoOnce false :!label _label_6
                (:Completed
                  (Components|Animation|PlayAnimation (Variables|Default|GetSKM_SingleDoor_Animated) "/Game/SciFi_Factory/SkeletonMeshes/SKM_SingleDoor_Close_Front.SKM_SingleDoor_Close_Front" false)
                  (Variables|Default|SetWhichSideOpened? "Closed")
                  (Utilities|FlowControl|Delay 1.0)
                  (Rendering|SetVisibility (Variables|Default|GetWidget_Line_Front) true false)
                  (goto _label_6 Reset))))))))))

(fn ConstructionScript
  (bind _widget_line_front (Variables|Default|GetWidget_Line_Front))
  (bind _returnvalue (Rendering|Material|CreateDynamicMaterialInstance (Variables|Default|GetSKM_SingleDoor_Animated) 1 "/Game/SciFi_Factory/Materials/MI_DoorPlastic.MI_DoorPlastic" "" :!class /Script/Engine.PrimitiveComponent))
  (Rendering|Material|SetVectorParameterValue _returnvalue "Color Multiply" (Variables|Default|GetDoorColor) :!class /Script/Engine.MaterialInstanceDynamic)
  (if (Variables|Default|GetIsLocked?)
    (Rendering|SetVisibility _widget_line_front false false)
    (Rendering|SetVisibility (Variables|Default|GetWidget_DoorLocked_Front) true false)
    (else
      (Rendering|SetVisibility _widget_line_front true false)
      (Rendering|SetVisibility (Variables|Default|GetWidget_DoorLocked_Back) false false)))
  (if (Variables|Default|GetReset)
    (Variables|Default|SetDoorColor "(R=0.187821,G=0.187821,B=0.187821,A=0.000000)")))

(fn ClosetheDoor
  (if (not (or (Utilities|Enum|Equal(Enum) (Variables|Default|GetWhichSideOpened?) "Closed") (== (Variables|Default|GetDontCloseDoor?) true)))
    (if (Utilities|Enum|Equal(Enum) (Variables|Default|GetWhichSideOpened?) "Front")
      (Utilities|FlowControl|DoOnce false :!label _label
        (:Completed
          (Components|Animation|PlayAnimation (Variables|Default|GetSKM_SingleDoor_Animated) "/Game/SciFi_Factory/SkeletonMeshes/SKM_SingleDoor_Close_Front.SKM_SingleDoor_Close_Front" false)
          (Variables|Default|SetWhichSideOpened? "Closed")
          (Rendering|SetVisibility (Variables|Default|GetWidget_Line_Front) true false)
          (goto _label Reset)))
      (else
        (Utilities|FlowControl|DoOnce false :!label _label_2
          (:Completed
            (Components|Animation|PlayAnimation (Variables|Default|GetSKM_SingleDoor_Animated) "/Game/SciFi_Factory/SkeletonMeshes/SKM_SingleDoor_Close_Back.SKM_SingleDoor_Close_Back" false)
            (Variables|Default|SetWhichSideOpened? "Closed")
            (Rendering|SetVisibility (Variables|Default|GetWidget_Line_Front) true false)
            (goto _label_2 Reset)))))))