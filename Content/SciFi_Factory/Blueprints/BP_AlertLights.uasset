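; BP_AlertLights is a spinning alarm light prop for the sci-fi factory environment.
; A looping timer calls Rotate at an interval set by Speed, adding a fixed yaw step to the inner alarm light mesh.
; The construction script and BeginPlay both apply the configurable color and intensity to the LSpinAlert light component.
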(event Custom|Rotate
  (Transformation|AddLocalRotation (Variables|Default|GetSM_AlarmLight_Inside) "0.000000,5.000000,0.000000" false false))

(event EventBeginPlay
  (bind _l_spinalert (Variables|Default|GetL_SpinAlert))
  (Utilities|Time|SetTimerbyFunctionName 0 "Rotate" (Variables|Default|GetSpeed) true)
  (Rendering|Components|Light|SetLightColor _l_spinalert (Math|Conversions|ToLinearColor(Color) (Variables|Default|GetLight%20Color)) true)
  (Rendering|Components|Light|SetIntensity _l_spinalert (Variables|Default|GetLight%20Intensity)))

(event Collision|EventActorBeginOverlap
  (params (OtherActor :type Actor%20Object%20Reference)))

(event EventTick
  (params (DeltaSeconds :type Float%20%28single-precision%29)))

(fn ConstructionScript
  (bind _l_spinalert (Variables|Default|GetL_SpinAlert))
  (Rendering|Components|Light|SetLightColor _l_spinalert (Math|Conversions|ToLinearColor(Color) (Variables|Default|GetLight%20Color)) true)
  (Rendering|Components|Light|SetIntensity _l_spinalert (Variables|Default|GetLight%20Intensity)))