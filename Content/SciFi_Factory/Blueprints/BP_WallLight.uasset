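; BP_WallLight is a configurable light fixture with a rect light and an emissive mesh that periodically pulses.
; The construction script applies the exposed light and material settings, and BeginPlay sets up a dynamic emissive material.
; A looping timer calls Pulse at an interval randomized once at BeginPlay.
; Pulse runs two timelines that animate light intensity and mesh emissive, restoring their base values on finish.
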(event Custom|Pulse
  (bind _sm_ceilinglight_01 (Variables|Default|GetSM_CeilingLight_01))
  (bind _rectlight (Variables|Default|GetRectLight))
  (Utilities|FlowControl|Sequence
    (:then_0
      (bind _newtrack_0 (Timeline|Timeline PlayFromStart)
        (:Update
          (Rendering|Components|Light|SetIntensity _rectlight _newtrack_0))
        (:Finished
          (Rendering|Components|Light|SetIntensity _rectlight (Variables|Default|GetLightINtensity)))))
    (:then_1
      (bind _newtrack_0_2 (Timeline|LightPulse PlayFromStart)
        (:Update
          (Rendering|Material|SetScalarParameterValueonMaterials _sm_ceilinglight_01 "Emissive" _newtrack_0_2))
        (:Finished
          (Rendering|Material|SetScalarParameterValueonMaterials _sm_ceilinglight_01 "Emissive" (Variables|Default|GetLight_Emissive)))))))

(event EventBeginPlay
  (bind _sm_ceilinglight_01 (Variables|Default|GetSM_CeilingLight_01))
  (Rendering|Material|SetScalarParameterValueonMaterials _sm_ceilinglight_01 "Emissive" (Variables|Default|GetLight_Emissive))
  (bind _returnvalue (Rendering|Material|CreateDynamicMaterialInstance _sm_ceilinglight_01 4 (Variables|Default|GetEmissiveMaterial) "None" :!class /Script/Engine.PrimitiveComponent))
  (Rendering|Material|SetVectorParameterValue _returnvalue "Emissive Color" (Variables|Default|GetEmissiveColor) :!class /Script/Engine.MaterialInstanceDynamic)
  (Rendering|Material|SetVectorParameterValue _returnvalue "Color" (Variables|Default|GetTurnOffColor) :!class /Script/Engine.MaterialInstanceDynamic)
  (Utilities|Time|SetTimerbyFunctionName 0 "Pulse" (Math|Conversions|ToFloat(Integer) (Math|Random|RandomIntegerinRange (Variables|Default|GetMinRandom) (Variables|Default|GetMaxRandom))) true))

(event Collision|EventActorBeginOverlap
  (params (OtherActor :type Actor%20Object%20Reference)))

(event EventTick
  (params (DeltaSeconds :type Float%20%28single-precision%29)))

(fn ConstructionScript
  (bind _emissivematerial (Variables|Default|GetEmissiveMaterial))
  (bind _light_emissive (Variables|Default|GetLight_Emissive))
  (bind _rectlight (Variables|Default|GetRectLight))
  (Rendering|Material|SetMaterialbyName (Variables|Default|GetSM_CeilingLight_01) "Light" _emissivematerial)
  (Rendering|Material|SetScalarParameterValueonMaterials (Variables|Default|GetSM_CeilingLight_01) "Emissive" _light_emissive)
  (bind _returnvalue (Rendering|Material|CreateDynamicMaterialInstance (Variables|Default|GetSM_CeilingLight_01) 4 _emissivematerial "" :!class /Script/Engine.PrimitiveComponent))
  (Rendering|Material|SetVectorParameterValue _returnvalue "Emissive Color" (Variables|Default|GetEmissiveColor) :!class /Script/Engine.MaterialInstanceDynamic)
  (Rendering|Material|SetScalarParameterValue _returnvalue "Emissive" _light_emissive :!class /Script/Engine.MaterialInstanceDynamic)
  (Rendering|Components|Light|SetIntensity _rectlight (Variables|Default|GetLightINtensity))
  (Rendering|Components|Light|SetLightColor _rectlight (Variables|Default|GetLightColor) true)
  (Class|LightComponent|SetTemperature _rectlight (Variables|Default|GetLightTemperature))
  (Class|LightComponent|SetIndirectLightingIntensity _rectlight (Variables|Default|GetLightINdirectIntensity))
  (Rendering|Lighting|SetAttenuationRadius _rectlight (Variables|Default|GetLightAttenuation)))